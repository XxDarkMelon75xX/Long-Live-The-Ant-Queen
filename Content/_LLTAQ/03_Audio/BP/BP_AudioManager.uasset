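; BP_AudioManager controls master, music and SFX volume levels for the game.
; Each setter applies a volume override on its own sound mix and sound class, then pushes that mix.
; On BeginPlay it also creates the WBP_Options widget and adds it to the viewport.
; GetMasterVolume is an empty stub.
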(event `self.ReceiveBeginPlay`
  (bind _returnvalue (`|CreateWidget` "/Game/_LLTAQ/06_UI/WBP_Options.WBP_Options_C"))
  (`UserWidget.AddToViewport` _returnvalue 0))

(fn `GetMasterVolume`)

(fn `SetMasterVolume`
  (params (Volume :type "Float (single-precision)"))
  (`GameplayStatics.SetSoundMixClassOverride` "/Game/_LLTAQ/03_Audio/SoundClassMix/MasterSoundMix.MasterSoundMix" "/Game/_LLTAQ/03_Audio/SoundClass/MasterSoundClass.MasterSoundClass" Volume)
  (`GameplayStatics.PushSoundMixModifier` "/Game/_LLTAQ/03_Audio/SoundClassMix/MasterSoundMix.MasterSoundMix"))

(fn `SetMusicVolume`
  (params (Volume :type "Float (single-precision)"))
  (`GameplayStatics.SetSoundMixClassOverride` "/Game/_LLTAQ/03_Audio/SoundClassMix/MusicSoundMix.MusicSoundMix" "/Game/_LLTAQ/03_Audio/SoundClass/MusicSoundClass.MusicSoundClass" Volume)
  (`GameplayStatics.PushSoundMixModifier` "/Game/_LLTAQ/03_Audio/SoundClassMix/MusicSoundMix.MusicSoundMix"))

(fn `SetSFXVolume`
  (params (Volume :type "Float (single-precision)"))
  (`GameplayStatics.SetSoundMixClassOverride` "/Game/_LLTAQ/03_Audio/SoundClassMix/SFXSoundMix.SFXSoundMix" "/Game/_LLTAQ/03_Audio/SoundClass/SFXSoundClass.SFXSoundClass" Volume)
  (`GameplayStatics.PushSoundMixModifier` "/Game/_LLTAQ/03_Audio/SoundClassMix/SFXSoundMix.SFXSoundMix"))

(fn `UserConstructionScript`)