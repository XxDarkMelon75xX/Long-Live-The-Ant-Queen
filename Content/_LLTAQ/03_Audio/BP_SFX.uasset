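; BP_SFX is a placeable sound-effect actor that plays an assigned SFX asset through its Audio component.
; The construction script applies the volume multiplier, and the sound can start automatically on BeginPlay or be triggered and stopped through PlaySFX and StopSFX.
; When looping is enabled, it replays after each finish following a random delay between minimum and maximum loop times, spacing out repeats.
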(event `self.ReceiveBeginPlay`
  (if (`self.PlayOnAwake`)
    (`self.PlaySFX`)))

(event `self.Audio.OnAudioFinished`
  (if (`self.IsLooping`)
    (`KismetSystemLibrary.Delay` (`KismetMathLibrary.RandomFloatInRange` (`self.MinLoopTime`) (`self.MaxLoopTime`)))
    (`self.PlaySFX`)))

(fn `PlaySFX`
  (bind _audio (`self.Audio`))
  (`AudioComponent.SetSound` _audio (`self.SFX`))
  (`AudioComponent.Play` _audio 0.0))

(fn `SetVolume`
  (`AudioComponent.SetVolumeMultiplier` (`self.Audio`) (`self.New Volume Multiplier`)))

(fn `StopSFX`
  (`AudioComponent.Stop` (`self.Audio`)))

(fn `UserConstructionScript`
  (`self.SetVolume`))