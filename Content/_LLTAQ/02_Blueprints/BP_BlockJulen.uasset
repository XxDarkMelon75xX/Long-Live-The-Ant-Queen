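; A pushable block that RTS ant units carry along a spline once enough of them occupy its hold points.
; It spawns a ring of BP_HoldPoints at BeginPlay, previewed as billboards by the construction script, and assigns interacting units to free ones.
; Reaching the required ant count makes them unselectable and starts a timeline move, freeing them when finished or blocked.
; Hover swaps overlay materials and reveals a bobbing ant-count widget.
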(event `self.ReceiveBeginPlay`
  (bind (_relativelocation_x _relativelocation_y _relativelocation_z) (`KismetMathLibrary.BreakVector` (`SceneComponent.RelativeLocation` (`self.Widget`))))
  (`self.CreateHoldPoints`)
  (`MeshComponent.SetOverlayMaterial` (`self.Cube`) "/Game/_LLTAQ/07_Materials/M_Outline.M_Outline")
  (set `self.BaseZ` _relativelocation_z))

(event `self.Interact`
  (params (Interactor :type "Actor Object Reference"))
  (bind _asbp_rtsunit (cast `/Game/_LLTAQ/02_Blueprints/BP_RTSUnit` Interactor))
  (bind _here (`self.IsAssigned` _asbp_rtsunit))
  (if (not _here)
    (bind _holdpoint (`self.GetFreeHoldPoint`))
    (`/Engine/EditorBlueprintResources/StandardMacros.IsValid` _holdpoint
      (:`Is Valid`
        (`/Game/_LLTAQ/02_Blueprints/BP_HoldPoint.AssignUnit` _holdpoint _asbp_rtsunit)
        (`/Game/_LLTAQ/02_Blueprints/BP_RTSUnit.AssignHoldPoint` _asbp_rtsunit _holdpoint)))))

(event `self.ReceiveTick`
  (params (DeltaSeconds :type "Float (single-precision)"))
  (set `self.ElapsedTime` (+ DeltaSeconds (`self.ElapsedTime`)))
  (`SceneComponent.K2_SetRelativeLocation` (`self.Widget`) (`KismetMathLibrary.MakeVector` 0.0 0.0 (+ (* (`self.FloatAmplitude`) (`KismetMathLibrary.Sin` (* (`self.ElapsedTime`) (`self.FloatSpeed`)))) (`self.BaseZ`))) true false))

(event `Move`
  (bind _spline (`/Game/_LLTAQ/02_Blueprints/BP_Path.Spline` (`self.Spline`)))
  (if (not (`self.HasMoved`))
    (`self.ReserveAllAnts`)
    (`TimelineComponent.SetPlayRate` (`self.T_Move`) (/ 1.0 (`self.TimeToComplete`)))
    (bind (_direction _t_move_track) (`Timeline|T_Move` :`NewTime` (`self.DistanceTraveled`) :!label _label)
      (:`Update`
        (set `self.DistanceTraveled` _t_move_track)
        (bind _returnvalue (`KismetMathLibrary.Lerp` 0.0 (`SplineComponent.GetSplineLength` (`/Game/_LLTAQ/02_Blueprints/BP_Path.Spline` (`self.Spline`))) _t_move_track))
        (bind _sweephitresult (`self.K2_SetActorLocationAndRotation` (`SplineComponent.GetLocationAtDistanceAlongSpline` _spline _returnvalue "World") (`SplineComponent.GetRotationAtDistanceAlongSpline` _spline _returnvalue "World") true))
        (if (`GameplayStatics.BreakHitResult` _sweephitresult)
          (`self.FreeAllAnts`)
          (goto _label :!via `Stop`)))
      (:`Finished`
        (set `self.HasMoved` true)
        (set `self.Hovered` false)
        (`self.FreeAllAnts`)
        (`MeshComponent.SetOverlayMaterial` (`self.Cube`) null)))))

(event `self.Cube.OnBeginCursorOver`
  (params (TouchedComponent :type "PrimitiveComponent Object Reference"))
  (if (not (`self.HasMoved`))
    (set `self.Hovered` true)
    (`MeshComponent.SetOverlayMaterial` (`self.Cube`) "/Game/_LLTAQ/07_Materials/M_Hover.M_Hover")
    (`SceneComponent.SetVisibility` (`self.Widget`) true false)))

(event `self.Cube.OnEndCursorOver`
  (params (TouchedComponent :type "PrimitiveComponent Object Reference"))
  (if (not (`self.HasMoved`))
    (set `self.Hovered` false)
    (`MeshComponent.SetOverlayMaterial` (`self.Cube`) "/Game/_LLTAQ/07_Materials/M_Outline.M_Outline")
    (if (== (`self.CurrentAnts`) 0)
      (`SceneComponent.SetVisibility` (`self.Widget`) false false))))

(fn `AddAnt`
  (`/Engine/EditorBlueprintResources/StandardMacros.IncrementInt` (`self.CurrentAnts`)
    (:`  `
      (`self.CheckMovable`)
      (bind _aswbp_block_info (cast `/Game/_LLTAQ/06_UI/WBP_BlockInfo` (`WidgetComponent.GetWidget` (`self.Widget`))))
      (`/Game/_LLTAQ/06_UI/WBP_BlockInfo.UpdateText` _aswbp_block_info (`self.CurrentAnts`) (`self.RequiredAnts`))
      (`SceneComponent.SetVisibility` (`self.Widget`) true false))))

(fn `CheckMovable`
  (if (>= (`self.CurrentAnts`) (`self.RequiredAnts`))
    (set `self.bMovable` true)
    (`self.Move`)
    (else
      (set `self.bMovable` false))))

(fn `CreateHoldPoints`
  (locals (AngleStep :type "Float (double-precision)" :default 0.0) (Angle :type "Float (double-precision)") (X :type "Float (double-precision)") (Y :type "Float (double-precision)") (Z :type "Float (double-precision)" :default 0.0))
  (set `local.AngleStep` (/ 360.0 (`KismetMathLibrary.Conv_IntToDouble` (`self.RequiredAnts`))))
  (for _index (range (`self.RequiredAnts`))
    (set `local.Angle` (+ (* _index (`local.AngleStep`)) (`self.SurroundRotationOffset`)))
    (set `local.X` (* (`KismetMathLibrary.DegCos` (`local.Angle`)) (`self.SurroundRadius`)))
    (set `local.Y` (* (`KismetMathLibrary.DegSin` (`local.Angle`)) (`self.SurroundRadius`)))
    (set `local.Z` (`self.SurroundHeightOffset`))
    (bind _returnvalue (`|SpawnActorFromClass` "/Game/_LLTAQ/02_Blueprints/BP_HoldPoint.BP_HoldPoint_C" (`SceneComponent.K2_GetComponentToWorld` (`self.HoldPointsRoot`)) "Undefined" "MultiplyWithRoot" null null))
    (`KismetArrayLibrary.Array_Add` (`self.HoldPoints`) _returnvalue)
    (bind _rootcomponent (`Actor.RootComponent` _returnvalue))
    (`SceneComponent.K2_AttachToComponent` _rootcomponent (`self.HoldPointsRoot`) "None" "KeepRelative" "KeepRelative" "KeepRelative" true)
    (`SceneComponent.K2_SetRelativeLocation` _rootcomponent (`KismetMathLibrary.MakeVector` (`local.X`) (`local.Y`) (`local.Z`)) false false)
    (set `/Game/_LLTAQ/02_Blueprints/BP_HoldPoint.ParentBlock` self _returnvalue)
    (set `/Game/_LLTAQ/02_Blueprints/BP_HoldPoint.FreeLocationPoint` (`self.ExitPoint`) _returnvalue)))

(fn `DragSelectResult`
  (params (SelectedActors :type "Array of Actor Object Reference (by ref)"))
  (returns (NewParam :type Boolean))
  (return false))

(fn `fgezomkgfezkhb`
  (returns (NewParam :type Boolean))
  (return false))

(fn `FreeAllAnts`
  (for _array_element (`self.HoldPoints`)
    (`/Game/_LLTAQ/02_Blueprints/BP_RTSUnit.FreeHoldPoint` (`/Game/_LLTAQ/02_Blueprints/BP_HoldPoint.CurrentUnit` _array_element))))

(fn `GetFreeHoldPoint`
  (returns (HoldPoint :type "/Game/_LLTAQ/02_Blueprints/BP_HoldPoint Object Reference"))
  (for _array_element (`self.HoldPoints`)
    (if (not (`/Game/_LLTAQ/02_Blueprints/BP_HoldPoint.bIsOccupied` _array_element))
      (return _array_element)))
  (return null))

(fn `GetInteractLocation`
  (returns (Location :type "Vector Structure"))
  (return (`SceneComponent.K2_GetComponentLocation` (`self.InteractLocation`))))

(fn `IsAssigned`
  (params (Unit :type "/Game/_LLTAQ/02_Blueprints/BP_RTSUnit Object Reference"))
  (returns (Here :type Boolean))
  (for _array_element (`self.HoldPoints`)
    (if (== (`/Game/_LLTAQ/02_Blueprints/BP_HoldPoint.CurrentUnit` _array_element) Unit)
      (return true)))
  (return false))

(fn `PassSelectedUnits`
  (returns (Actors :type "Array of Actor Object Reference"))
  (return))

(fn `RemoveAnt`
  (`/Engine/EditorBlueprintResources/StandardMacros.DecrementInt` (`self.CurrentAnts`)
    (:`  `
      (`self.CheckMovable`)
      (bind _aswbp_block_info (cast `/Game/_LLTAQ/06_UI/WBP_BlockInfo` (`WidgetComponent.GetWidget` (`self.Widget`))))
      (`/Game/_LLTAQ/06_UI/WBP_BlockInfo.UpdateText` _aswbp_block_info (`self.CurrentAnts`) (`self.RequiredAnts`))
      (if (and (not (`self.Hovered`)) (== (`self.CurrentAnts`) 0))
        (`SceneComponent.SetVisibility` (`self.Widget`) false false)))))

(fn `ReserveAllAnts`
  (for _array_element (`self.HoldPoints`)
    (set `/Game/_LLTAQ/02_Blueprints/BP_RTSUnit.bSelectable` false (`/Game/_LLTAQ/02_Blueprints/BP_HoldPoint.CurrentUnit` _array_element))))

(fn `UnselectAllAnts`
  (for _array_element (`self.HoldPoints`)
    (set `/Game/_LLTAQ/02_Blueprints/BP_RTSUnit.bSelectable` false (`/Game/_LLTAQ/02_Blueprints/BP_HoldPoint.CurrentUnit` _array_element))))

(fn `UserConstructionScript`
  (locals (AngleStep :type "Float (double-precision)") (Angle :type "Float (double-precision)") (X :type "Float (double-precision)") (Y :type "Float (double-precision)") (Z :type "Float (double-precision)"))
  (set `local.AngleStep` (/ 360.0 (`KismetMathLibrary.Conv_IntToDouble` (`self.RequiredAnts`))))
  (for _index (range (`self.RequiredAnts`))
    (set `local.Angle` (+ (* _index (`local.AngleStep`)) (`self.SurroundRotationOffset`)))
    (set `local.X` (* (`KismetMathLibrary.DegCos` (`local.Angle`)) (`self.SurroundRadius`)))
    (set `local.Y` (* (`KismetMathLibrary.DegSin` (`local.Angle`)) (`self.SurroundRadius`)))
    (set `local.Z` (`self.SurroundHeightOffset`))
    (bind _returnvalue (`AddComponent|NODE_AddBillboardComponent-0`))
    (`SceneComponent.K2_SetRelativeLocation` _returnvalue (`KismetMathLibrary.MakeVector` (`local.X`) (`local.Y`) (`local.Z`)) false false)))