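; Selectable RTS ant unit that takes move, follow and interact orders through AI MoveTo.
; Follow reissues the move on each arrival while the followed unit is still moving.
; Overlapping the interact target attaches the unit to a free interact point with collision off; new orders free it and teleport it to any exit point.
; Also handles outline selection highlighting, selection lockout via the player controller, and a timed burning animation.
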(event `InteractWithActor`
  (params (Actor :type "Actor Object Reference"))
  (`self.DetachFromInteractPoint`)
  (`MovementComponent.StopMovementImmediately` (`self.CharacterMovement`))
  (set `self.InteractActor` Actor)
  (set `self.bIsMoving` true)
  (`|AIMoveTo` self (0.0 0.0 0.0) Actor
    (:`OnSuccess`
      (set `self.bIsMoving` false))))

(event `MoveToLocation`
  (params (Location :type "Vector Structure"))
  (`self.DetachFromInteractPoint`)
  (`MovementComponent.StopMovementImmediately` (`self.CharacterMovement`))
  (set `self.bIsMoving` true)
  (set `self.InteractActor` null)
  (`|AIMoveTo` self Location null
    (:`OnSuccess`
      (set `self.bIsMoving` false))))

(event `FollowUnit`
  (params (UnitToFollow :type "/Game/_LLTAQ/02_Blueprints/BP_RTSUnit Object Reference"))
  (`self.DetachFromInteractPoint`)
  (`MovementComponent.StopMovementImmediately` (`self.CharacterMovement`))
  (set `self.bIsMoving` true)
  (set `self.Unit to Follow` UnitToFollow)
  (set `self.InteractActor` null)
  (`self.FollowUnitLoop`))

(event `FollowUnitLoop`
  (`|AIMoveTo` self (0.0 0.0 0.0) (`self.Unit to Follow`) 50.0
    (:`OnSuccess`
      (if (`/Game/_LLTAQ/02_Blueprints/BP_RTSUnit.bIsMoving` (`self.Unit to Follow`))
        (`self.FollowUnitLoop`)
        (else
          (set `self.bIsMoving` false))))))

(event `self.CapsuleComponent.OnComponentBeginOverlap`
  (params (OverlappedComponent :type "PrimitiveComponent Object Reference") (OtherActor :type "Actor Object Reference") (OtherComp :type "PrimitiveComponent Object Reference") (OtherBodyIndex :type Integer) (bFromSweep :type Boolean) (SweepResult :type "HitResult Structure (by ref)"))
  (if (== OtherActor (`self.InteractActor`))
    (`MovementComponent.StopMovementImmediately` (`self.CharacterMovement`))
    (set `self.bIsMoving` false)
    (bind _point (message `/Game/_LLTAQ/02_Blueprints/BPI_Interaction.GetFreeInteractPoint` (`self.InteractActor`)))
    (`/Engine/EditorBlueprintResources/StandardMacros.IsValid` _point
      (:`Is Valid`
        (set `self.InteractPoint` _point)
        (`self.AttachToInteractPoint`)))))

(event `PlayFireAnimation`
  (bind _asab_ant (cast `/Game/_LLTAQ/05_Characters/Ant/ant/source/Anims/AB_Ant` (`SkeletalMeshComponent.GetAnimInstance` (`self.Mesh`))))
  (set `/Game/_LLTAQ/05_Characters/Ant/ant/source/Anims/AB_Ant.IsBurning` true _asab_ant)
  (`KismetSystemLibrary.Delay` 2.5)
  (set `/Game/_LLTAQ/05_Characters/Ant/ant/source/Anims/AB_Ant.IsBurning` false _asab_ant))

(fn `AttachToInteractPoint`
  (`self.DisableCollision`)
  (`self.K2_SetActorLocationAndRotation` (`self.K2_GetActorLocation` (`self.InteractPoint`)) (struct) false true)
  (`self.K2_AttachToActor` (`self.InteractPoint`) "None" "KeepWorld" "KeepRelative" "KeepWorld")
  (`/Game/_LLTAQ/02_Blueprints/BP_InteractPoint.AssignUnit` (`self.InteractPoint`) self))

(fn `DeselectUnit`
  (`MeshComponent.SetOverlayMaterial` (`self.Mesh`) null))

(fn `DetachFromInteractPoint`
  (bind _interactpoint (`self.InteractPoint`))
  (`/Engine/EditorBlueprintResources/StandardMacros.IsValid` _interactpoint
    (:`Is Valid`
      (`/Game/_LLTAQ/02_Blueprints/BP_InteractPoint.FreeUnit` _interactpoint)
      (`self.K2_DetachFromActor` self "KeepWorld" "KeepRelative" "KeepWorld")
      (bind _arrow (message `/Game/_LLTAQ/02_Blueprints/BPI_Interaction.GetExitPoint` (`self.InteractActor`)))
      (`/Engine/EditorBlueprintResources/StandardMacros.IsValid` _arrow
        (:`Is Valid`
          (`self.K2_SetActorLocation` (`SceneComponent.K2_GetComponentLocation` _arrow) false true))
        (:`Is Not Valid`
          _))
      (set `self.InteractPoint` null)
      (set `self.InteractActor` null)
      (set `self.bSelectable` true)
      (`self.EnableCollision`))))

(fn `DisableCollision`
  (`PrimitiveComponent.SetCollisionEnabled` (`self.CapsuleComponent`) "NoCollision"))

(fn `EnableCollision`
  (`PrimitiveComponent.SetCollisionEnabled` (`self.CapsuleComponent`) "QueryAndPhysics"))

(fn `PreventSelection`
  (set `self.bSelectable` false)
  (bind _asbp_rtsplayer_controller (cast `/Game/_LLTAQ/02_Blueprints/BP_RTSPlayerController` (`GameplayStatics.GetPlayerController` 0)))
  (`/Game/_LLTAQ/02_Blueprints/BP_RTSPlayerController.RemoveAntFromCollection` _asbp_rtsplayer_controller self))

(fn `SelectUnit`
  (`MeshComponent.SetOverlayMaterial` (`self.Mesh`) "/Game/_LLTAQ/07_Materials/M_OutlineBlue.M_OutlineBlue"))

(fn `UserConstructionScript`)