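; RTS player controller for commanding ant units with the mouse and moving an angled, zoomable camera pawn.
; Clicks select units via an upward sphere trace with a modifier for multi-select, while drags update the HUD's selection box.
; Move orders send the closest unit to the goal and chain the others to follow one another.
; Clicks on a hovered interact actor dispatch units, capped by the ant count it requests.
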(event `self.ReceiveBeginPlay`
  (`|ExecutionSequence`
    (:`then_0`
      (bind _asbp_rtspawn (cast `/Game/_LLTAQ/02_Blueprints/BP_RTSPawn` (`self.K2_GetPawn`)))
      (bind _orthowidth (`CameraComponent.OrthoWidth` (`/Game/_LLTAQ/02_Blueprints/BP_RTSPawn.Camera` _asbp_rtspawn)))
      (set `self.Camera Zoom` _orthowidth)
      (set `self.ControlledPawn` _asbp_rtspawn)
      (set `self.DefaultZoom` _orthowidth))
    (:`then_1`
      (`EnhancedInputSubsystemInterface.AddMappingContext` (subsystem `EnhancedInputLocalPlayerSubsystem`) "/Game/_LLTAQ/04_Inputs/IMC_Mouse.IMC_Mouse" 0 (struct)))
    (:`then_2`
      (`self.GetRTSHUD`))))

(event `EnhancedInput|/Game/_LLTAQ/04_Inputs/Actions/IA_RTS_SelectHold`
  (params (ActionValue :type Boolean) (ElapsedSeconds :type "Float (double-precision)") (TriggeredSeconds :type "Float (double-precision)") (InputAction :type "InputAction Object Reference" :default "/Game/_LLTAQ/04_Inputs/Actions/IA_RTS_SelectHold.IA_RTS_SelectHold"))
  (bind (_startingselectionposition_x _startingselectionposition_y) (`KismetMathLibrary.BreakVector2D` (`self.StartingSelectionPosition`)))
  ;[0.15 0.15 0.15 0.502] Selection Logic for Mouse - Select / Drag Select on Hold
  (:`Triggered`
    (bind _mouse_pos (`self.GetMouseLocation`))
    (`/Game/_LLTAQ/02_Blueprints/BP_RTSHUD.DragUpdate` (`self. RTSHUD`) (`self.StartingSelectionPosition`) (`KismetMathLibrary.MakeVector2D` (- (`KismetMathLibrary.BreakVector2D` _mouse_pos) _startingselectionposition_x) (- (`.Y` (`KismetMathLibrary.BreakVector2D` _mouse_pos)) _startingselectionposition_y)) (`KismetMathLibrary.MakeVector2D` (`KismetMathLibrary.BreakVector2D` _mouse_pos) (`.Y` (`KismetMathLibrary.BreakVector2D` _mouse_pos))) true))
  (:`Started`
    (bind _mouse_pos_2 (`self.GetMouseLocation`))
    (set `self.StartingSelectionPosition` _mouse_pos_2))
  (:`Canceled`
    (`/Game/_LLTAQ/02_Blueprints/BP_RTSHUD.DragUpdate` (`self. RTSHUD`) (0.0 0.0) (0.0 0.0) (0.0 0.0) false :!label _label))
  (:`Completed`
    (goto _label)))

(event `EnhancedInput|/Game/_LLTAQ/04_Inputs/Actions/IA_RTS_MoveCamera`
  (params (ActionValue :type "Vector2D Structure") (ElapsedSeconds :type "Float (double-precision)") (TriggeredSeconds :type "Float (double-precision)") (InputAction :type "InputAction Object Reference" :default "/Game/_LLTAQ/04_Inputs/Actions/IA_RTS_MoveCamera.IA_RTS_MoveCamera"))
  (bind (_returnvalue_roll _returnvalue_pitch _returnvalue_yaw) (`KismetMathLibrary.BreakRotator` (`self.GetControlRotation`)))
  (bind (_returnvalue_roll_2 _returnvalue_pitch_2 _returnvalue_yaw_2) (`KismetMathLibrary.BreakRotator` (`self.GetControlRotation`)))
  (bind _controlledpawn (`self.ControlledPawn`))
  ;[0.15 0.15 0.15 0.502] Camera Logic
  ;;[0.15 0.15 0.15 0.502] Spectator Pawn Movement - our pawn is essentially a floating fixed angle camera. Because our view is 3/4, we're actually moving diagonally when it looks like we're moving straight
  (:`Triggered`
    (`Pawn.AddMovementInput` _controlledpawn (`KismetMathLibrary.GetForwardVector` (`KismetMathLibrary.MakeRotator` _returnvalue_roll 0.0 _returnvalue_yaw)) (+ ActionValue_X ActionValue_Y) false)
    (`Pawn.AddMovementInput` _controlledpawn (`KismetMathLibrary.GetRightVector` (`KismetMathLibrary.MakeRotator` 0.0 0.0 _returnvalue_yaw_2)) (- ActionValue_X ActionValue_Y) false)))

(event `EnhancedInput|/Game/_LLTAQ/04_Inputs/Actions/IA_RTS_SelectClick`
  (params (ActionValue :type Boolean) (ElapsedSeconds :type "Float (double-precision)") (TriggeredSeconds :type "Float (double-precision)") (InputAction :type "InputAction Object Reference" :default "/Game/_LLTAQ/04_Inputs/Actions/IA_RTS_SelectClick.IA_RTS_SelectClick"))
  ;[0.15 0.15 0.15 0.502] Selection Logic for Mouse - Select / Drag Select on Hold
  ;;[0.15 0.15 0.15 0.502] Click Select Input (fires off on Tap)
  (:`Completed`
    (`self.Do Selection Command - Mouse`)))

(event `Do Selection Command - Mouse`
  (bind (_hit _location) (`self.GetLocationUnderCursor`))
  (bind _cachedselection (`self.CachedSelection`))
  (bind _target_unit (`self.Target Unit`))
  (bind _target_unit_2 (`self.Target Unit`))
  (bind _controlled_units (`self.Controlled Units`))
  (if _hit
    (set `self.CachedSelection` _location)
    (bind _outhit (`KismetSystemLibrary.SphereTraceSingleForObjects` _cachedselection (+ _cachedselection (0.0 0.0 350.0)) (`self.RandomLocationRadius`) (`|MakeArray` "ObjectTypeQuery3" :!type "EObjectTypeQuery Enum") true)) ; Vertical sphere trace using the mouse location and interaction\nradius to catch any Z offset potential selectables
    (if (not (`self.SelectionModifier`))
      (`self.Do Deselect All Command`))
    (bind (_bblockinghit _binitialoverlap _time _distance _location_2 _impactpoint _normal _impactnormal _physmat _hitactor) (`GameplayStatics.BreakHitResult` _outhit))
    (if _bblockinghit
      (bind _asbp_rtsunit (cast `/Game/_LLTAQ/02_Blueprints/BP_RTSUnit` _hitactor))
      (set `self.Target Unit` _asbp_rtsunit)
      (if (`KismetArrayLibrary.Array_Contains` _controlled_units)
        (`KismetArrayLibrary.Array_RemoveItem` _controlled_units _target_unit)
        (`/Game/_LLTAQ/02_Blueprints/BP_RTSUnit.DeselectUnit` _target_unit)
        (else
          (`KismetArrayLibrary.Array_Add` _controlled_units _target_unit_2)
          (`/Game/_LLTAQ/02_Blueprints/BP_RTSUnit.SelectUnit` _target_unit_2))))))

(event `EnhancedInput|/Game/_LLTAQ/04_Inputs/Actions/IA_RTS_Zoom`
  (params (ActionValue :type "Float (double-precision)") (ElapsedSeconds :type "Float (double-precision)") (TriggeredSeconds :type "Float (double-precision)") (InputAction :type "InputAction Object Reference" :default "/Game/_LLTAQ/04_Inputs/Actions/IA_RTS_Zoom.IA_RTS_Zoom"))
  ;[0.15 0.15 0.15 0.502] Camera Logic
  ;;[0.15 0.15 0.15 0.502] Zoom Camera
  (:`Triggered`
    (bind _result (`/Engine/EditorBlueprintResources/StandardMacros.NegateFloat` ActionValue)
      (:`  `
        (bind _output_get (set `self.Camera Zoom` (`KismetMathLibrary.FClamp` (+ (* _result 100.0) (`self.Camera Zoom`)) 1000.0 2500.0)))
        (`/Game/_LLTAQ/02_Blueprints/BP_RTSPawn.ZoomModifier` (`self.ControlledPawn`) _output_get)))))

(event `EnhancedInput|/Game/_LLTAQ/04_Inputs/Actions/IA_RTS_SelectionModifier`
  (params (ActionValue :type Boolean) (ElapsedSeconds :type "Float (double-precision)") (TriggeredSeconds :type "Float (double-precision)") (InputAction :type "InputAction Object Reference" :default "/Game/_LLTAQ/04_Inputs/Actions/IA_RTS_SelectionModifier.IA_RTS_SelectionModifier"))
  ;[0.15 0.15 0.15 0.502] Selection Logic for Mouse - Select / Drag Select on Hold
  (:`Triggered`
    (set `self.SelectionModifier` ActionValue :!label _label_2))
  (:`Canceled`
    (goto _label_2))
  (:`Completed`
    (goto _label_2)))

(event `EnhancedInput|/Game/_LLTAQ/04_Inputs/Actions/IA_RTS_ResetCamera`
  (params (ActionValue :type Boolean) (ElapsedSeconds :type "Float (double-precision)") (TriggeredSeconds :type "Float (double-precision)") (InputAction :type "InputAction Object Reference" :default "/Game/_LLTAQ/04_Inputs/Actions/IA_RTS_ResetCamera.IA_RTS_ResetCamera"))
  ;[0.15 0.15 0.15 0.502] Camera Logic
  ;;[0.15 0.15 0.15 0.502] Zoom Camera
  (:`Triggered`
    (bind _output_get (set `self.Camera Zoom` (`self.DefaultZoom`)))
    (`/Game/_LLTAQ/02_Blueprints/BP_RTSPawn.ZoomModifier` (`self.ControlledPawn`) _output_get)))

(event `EnhancedInput|/Game/_LLTAQ/04_Inputs/Actions/IA_RTS_InteractClick`
  (params (ActionValue :type Boolean) (ElapsedSeconds :type "Float (double-precision)") (TriggeredSeconds :type "Float (double-precision)") (InputAction :type "InputAction Object Reference" :default "/Game/_LLTAQ/04_Inputs/Actions/IA_RTS_InteractClick.IA_RTS_InteractClick"))
  (bind (_hit _location) (`self.GetLocationUnderCursor`))
  (:`Completed`
    (`/Engine/EditorBlueprintResources/StandardMacros.IsValid` (`self.InteractActor`)
      (:`Is Valid`
        (`self.Do Move Units To Actor Command`))
      (:`Is Not Valid`
        (if (and (> (`KismetArrayLibrary.Array_Length` (`self.Controlled Units`)) 0) _hit)
          (set `self.Cached Interaction` _location)
          (`self.Do Move Units Command`))))))

(event `Do Move Units Command`
  (set `self.ClosestUnit` null)
  (bind _closest (`self.Get Closest Actor to Location` (`self.Controlled Units`) (`self.Cached Interaction`)))
  (bind _asbp_rtsunit (cast `/Game/_LLTAQ/02_Blueprints/BP_RTSUnit` _closest))
  (bind _output_get (set `self.ClosestUnit` _asbp_rtsunit))
  (bind _output_get_2 (set `self.PreviousUnit` _output_get))
  (`/Game/_LLTAQ/02_Blueprints/BP_RTSUnit.MoveToLocation` _output_get_2 (`self.Cached Interaction`))
  (for _array_element (`self.Controlled Units`)
    (if (not (== _array_element (`self.ClosestUnit`)))
      (`/Game/_LLTAQ/02_Blueprints/BP_RTSUnit.FollowUnit` _array_element (`self.PreviousUnit`))
      (set `self.PreviousUnit` _array_element))))

(event `Do Move Units To Actor Command`
  (bind _value (message `/Game/_LLTAQ/02_Blueprints/BPI_Interaction.GetAntsNeeded` (`self.InteractActor`)))
  (set `self.IndexForInteraction` 0)
  (set `self.AntNeededForInteraction` _value)
  (for _array_element (`self.Controlled Units`)
    (`/Game/_LLTAQ/02_Blueprints/BP_RTSUnit.InteractWithActor` _array_element (`self.InteractActor`))
    (bind _result (`/Engine/EditorBlueprintResources/StandardMacros.IncrementInt` (`self.IndexForInteraction`))
      (:`  `
        (if (>= _result (`self.AntNeededForInteraction`))
          (break))))))

(fn `2DVectorLength`
  (params (VectorA :type "Vector Structure") (VectorB :type "Vector Structure"))
  (returns (Length :type "Float (double-precision)"))
  (return (`KismetMathLibrary.VSize2D` (- (`KismetMathLibrary.MakeVector2D` VectorA_X VectorA_Y) (`KismetMathLibrary.MakeVector2D` VectorB_X VectorB_Y)))))

(fn `Do Deselect All Command`
  (bind _controlled_units (`self.Controlled Units`))
  (for _array_element _controlled_units
    (bind _asbp_rtsunit (cast `/Game/_LLTAQ/02_Blueprints/BP_RTSUnit` _array_element))
    (`/Game/_LLTAQ/02_Blueprints/BP_RTSUnit.DeselectUnit` _asbp_rtsunit))
  (`KismetArrayLibrary.Array_Clear` _controlled_units)
  (return))

(fn `Do Drag Scroll Command`
  (locals (WorkingPosition :type "Vector2D Structure"))
  (bind (_locationx _locationy) (`self.GetMousePosition`))
  (bind (_returnvalue_x _returnvalue_y) (`KismetMathLibrary.BreakVector2D` (- (`self.StartingInteractionPosition`) (`local.WorkingPosition`))))
  (set `local.WorkingPosition` (`KismetMathLibrary.MakeVector2D` _locationx _locationy))
  (`self.K2_AddActorWorldOffset` (`self.K2_GetPawn`) (* (`KismetMathLibrary.GreaterGreater_VectorRotator` (`KismetMathLibrary.MakeVector` _returnvalue_x _returnvalue_y) (struct :`Yaw` -45.0)) (`self.DragMultiplier`)) false false))

(fn `Get Closest Actor to Location`
  (params (ActorArray :type "Array of Actor Object Reference") (TargetLocation :type "Vector Structure"))
  (returns (Closest :type "Actor Object Reference"))
  (locals (`Out Actor` :type "Actor Object Reference") (`Closest Distance` :type "Float (double-precision)"))
  ; Process each actor on the list
  (set `local.Out Actor` null)
  (for _array_element ActorArray
    ; Have we selected a closest candidate already?
    (if (== (`local.Out Actor`) null)
      ; If we don't have an actor yet selected, choose the current one and set the closest distance.
      (bind _output_get (set `local.Out Actor` _array_element))
      (set `local.Closest Distance` (`KismetMathLibrary.Vector_DistanceSquared` (`self.K2_GetActorLocation` _output_get) (`local.TargetLocation`)))
      (else
        (bind _returnvalue (`KismetMathLibrary.Vector_DistanceSquared` (`self.K2_GetActorLocation` _array_element) (`local.TargetLocation`)))
        ; Check if the distance to the current actor is closer, and update the output actor and distance for the next chec.
        (if (< _returnvalue (`local.Closest Distance`))
          (set `local.Out Actor` _array_element)
          (set `local.Closest Distance` _returnvalue)))))
  ; When we're done, return the closest actor found
  (return (`local.Out Actor`)))

(fn `GetLocationUnderCursor`
  (returns (Hit :type Boolean) (Location :type "Vector Structure"))
  (bind (_bblockinghit _binitialoverlap _time _distance _location) (`GameplayStatics.BreakHitResult` (`self.GetHitResultUnderCursorByChannel` "TraceTypeQuery1")))
  (return _bblockinghit _location))

(fn `GetLocationUnderFinger`
  (returns (Hit :type Boolean) (Location :type "Vector Structure"))
  (bind (_bblockinghit _binitialoverlap _time _distance _location) (`GameplayStatics.BreakHitResult` (`self.GetHitResultUnderFingerByChannel` "Touch1" "TraceTypeQuery1" false)))
  (return _bblockinghit _location))

(fn `GetMouseLocation`
  (returns (`Mouse Pos` :type "Vector2D Structure"))
  (bind (_locationx _locationy) (`self.GetMousePosition` (`GameplayStatics.GetPlayerController` 0)))
  (return (`KismetMathLibrary.MakeVector2D` _locationx _locationy)))

(fn `GetRTSHUD`
  (bind _asbp_rtshud (cast `/Game/_LLTAQ/02_Blueprints/BP_RTSHUD` (`self.GetHUD`)))
  (set `self. RTSHUD` _asbp_rtshud))

(fn `GetSelectedUnits`
  (returns (Actors :type "Array of Actor Object Reference"))
  (return (`self.Controlled Units`)))

(fn `RemoveAntFromCollection`
  (params (Value :type "/Game/_LLTAQ/02_Blueprints/BP_RTSUnit Object Reference"))
  (if (`KismetArrayLibrary.Array_Contains` (`self.Controlled Units`) Value)
    (`KismetArrayLibrary.Array_RemoveItem` (`self.Controlled Units`) Value)
    (`/Game/_LLTAQ/02_Blueprints/BP_RTSUnit.DeselectUnit` Value)))

(fn `SetHoverActor`
  (params (Actor :type "Actor Object Reference") (bool :type Boolean))
  (if (== Actor (`self.InteractActor`))
    (if (not bool)
      (set `self.InteractActor` null))
    (elif bool
      (set `self.InteractActor` Actor))))

(fn `SetSelectedUnits`
  (params (Units :type "Array of Actor Object Reference"))
  (if (> (`KismetArrayLibrary.Array_Length` Units) 0)
    (`self.Do Deselect All Command`)
    (for _array_element Units
      (bind _asbp_rtsunit (cast `/Game/_LLTAQ/02_Blueprints/BP_RTSUnit` _array_element))
      (if (`/Game/_LLTAQ/02_Blueprints/BP_RTSUnit.bSelectable` _asbp_rtsunit)
        (`KismetArrayLibrary.Array_Add` (`self.Controlled Units`) _asbp_rtsunit)
        (`/Game/_LLTAQ/02_Blueprints/BP_RTSUnit.SelectUnit` _asbp_rtsunit)))))

(fn `UserConstructionScript`)