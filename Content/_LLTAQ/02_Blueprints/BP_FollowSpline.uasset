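; BP_FollowSpline is an actor that follows a referenced MovementSpline, looping continuously from BeginPlay.
; A Timeline, with play rate set from TimeToComplete, restarts from the beginning each time it finishes.
; Each update sets location and rotation, with sweep, from a distance along the spline.
; That distance's Lerp alpha is a constant 0 rather than a Timeline track, so it resolves to the spline's start.
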(event `StartMoving`
  (bind _spline (`/Game/_LLTAQ/02_Blueprints/BP_Path.Spline` (`self.MovementSpline`)))
  (bind _returnvalue (`KismetMathLibrary.Lerp` 0.0 (`SplineComponent.GetSplineLength` (`/Game/_LLTAQ/02_Blueprints/BP_Path.Spline` (`self.MovementSpline`)))))
  (`Timeline|Timeline` :!via `PlayFromStart`
    (:`Update`
      (`self.K2_SetActorLocationAndRotation` (`SplineComponent.GetLocationAtDistanceAlongSpline` _spline _returnvalue "World") (`SplineComponent.GetRotationAtDistanceAlongSpline` _spline _returnvalue "World") true))
    (:`Finished`
      (`self.StartMoving`))))

(event `self.ReceiveBeginPlay`
  (`TimelineComponent.SetPlayRate` (`self.Timeline`) (/ 1.0 (`self.TimeToComplete`)))
  (`self.StartMoving`))

(fn `UserConstructionScript`)