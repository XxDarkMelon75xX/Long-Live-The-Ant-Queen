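; BP_TutoCaller is a one-shot tutorial trigger actor that shows a configurable title and tip.
; It fires either after a delay on BeginPlay when CallOnStart is set, or when BP_RTSPawn hits its Box, which also prints a debug string.
; ShowTips flags itself as shown and passes the text to the UI of the level's BP_TutoManager, then the caller destroys itself.
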(event `self.ReceiveBeginPlay`
  (if (`self.CallOnStart`)
    (`KismetSystemLibrary.Delay` (`self.Delay`))
    (`self.ShowTips`)
    (`self.K2_DestroyActor`)))

(event `self.Box.OnComponentHit`
  (params (HitComponent :type "PrimitiveComponent Object Reference") (OtherActor :type "Actor Object Reference") (OtherComp :type "PrimitiveComponent Object Reference") (NormalImpulse :type "Vector Structure") (Hit :type "HitResult Structure (by ref)"))
  (if (not (`self.bShowedTips`))
    (cast `/Game/_LLTAQ/02_Blueprints/BP_RTSPawn` OtherActor)
    (`KismetSystemLibrary.PrintString` "Hello")
    (`self.ShowTips`)
    (`self.K2_DestroyActor`)))

(fn `ShowTips`
  (set `self.bShowedTips` true)
  (bind _returnvalue (`GameplayStatics.GetActorOfClass` "/Game/_LLTAQ/02_Blueprints/BP_TutoManager.BP_TutoManager_C"))
  (`/Engine/EditorBlueprintResources/StandardMacros.IsValid` _returnvalue
    (:`Is Valid`
      (bind _ui (`/Game/_LLTAQ/02_Blueprints/BP_TutoManager.UI` _returnvalue))
      (`/Game/_LLTAQ/06_UI/WBP_Tuto.SetNewTips` _ui (`self.Title`) (`self.Tips`))
      (`/Game/_LLTAQ/06_UI/WBP_Tuto.DisplayTips` _ui))))

(fn `UserConstructionScript`)