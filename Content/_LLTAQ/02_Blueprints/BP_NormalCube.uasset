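; BP_NormalCube is a cube actor that takes the place of a referenced Block once that block finishes moving.
; On BeginPlay it binds to the Block's end-move event if the reference is valid.
; The bound handler destroys the Block, unhides its own Cube component and, if the Physics flag is set, turns on physics simulation for it.
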(event `self.ReceiveBeginPlay`
  (`/Engine/EditorBlueprintResources/StandardMacros.IsValid` (`self.Block`)
    (:`Is Valid`
      (add `/Game/_LLTAQ/02_Blueprints/BP_Block.OnEndMove` (`self.Block`) (delegate `Destroy!!!!`)))))

(event `Destroy!!!!`
  (`self.K2_DestroyActor` (`self.Block`))
  (`SceneComponent.SetHiddenInGame` (`self.Cube`) false false)
  (if (`self.physics`)
    (`PrimitiveComponent.SetSimulatePhysics` (`self.Cube`) true)))

(fn `UserConstructionScript`)