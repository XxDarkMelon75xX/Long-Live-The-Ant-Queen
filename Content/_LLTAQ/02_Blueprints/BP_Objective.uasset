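; BP_Objective is an objective actor with a Cone component that bobs up and down continuously.
; BeginPlay stores the cone's starting world height as BaseZ.
; Tick accumulates elapsed time and teleports the cone to a sine offset around that height, keeping its current X and Y, with Speed setting the frequency and VerticalMovementLength the amplitude.
; It contains no objective or completion logic, only this animation.
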(event `self.ReceiveBeginPlay`
  (bind (_returnvalue_x _returnvalue_y _returnvalue_z) (`KismetMathLibrary.BreakVector` (`SceneComponent.K2_GetComponentLocation` (`self.Cone`))))
  (set `self.BaseZ` _returnvalue_z))

(event `self.ReceiveTick`
  (params (DeltaSeconds :type "Float (single-precision)"))
  (bind _cone (`self.Cone`))
  (bind (_returnvalue_x _returnvalue_y) (`KismetMathLibrary.BreakVector` (`SceneComponent.K2_GetComponentLocation` _cone)))
  (set `self.ElapsedTime` (+ DeltaSeconds (`self.ElapsedTime`)))
  (`SceneComponent.K2_SetWorldLocation` _cone (`KismetMathLibrary.MakeVector` _returnvalue_x _returnvalue_y (+ (* (`KismetMathLibrary.Sin` (* (`self.ElapsedTime`) (`self.Speed`))) (`self.VerticalMovementLength`)) (`self.BaseZ`))) false true))

(fn `UserConstructionScript`)