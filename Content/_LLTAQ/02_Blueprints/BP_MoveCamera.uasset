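; Scripted camera move actor that slides the RTS pawn's Cube to this actor's Arrow location, optionally auto-starting after a delay on BeginPlay.
; StartMoving disables player input and pawn wall collision, then lerps position on a timeline over TimeToComplete, restoring both when finished.
; The actor and timeline tick while paused, with a tiny CustomTimeDilation offset by a matching play-rate multiplier.
; SetGamePaused nodes are present but unconnected.
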(event `self.ReceiveBeginPlay`
  (bind _returnvalue (`GameplayStatics.GetActorOfClass` "/Game/_LLTAQ/02_Blueprints/BP_RTSPawn.BP_RTSPawn_C"))
  (set `self.Pawn` _returnvalue)
  (if (`self.CallOnStart`)
    (`KismetSystemLibrary.Delay` (`self.Delay`))
    (`self.StartMoving`)))

(event `StartMoving`
  (bind _returnvalue (`GameplayStatics.GetPlayerController` 0))
  (bind _returnvalue_2 (`GameplayStatics.GetPlayerController` 0))
  (bind _timelinemoving (`self.TimelineMoving`))
  (`self.DisableInput` _returnvalue _returnvalue)
  (`/Game/_LLTAQ/02_Blueprints/BP_RTSPawn.GoThroughWalls` (`self.Pawn`))
  (`self.SetTickableWhenPaused` true)
  (set `self.CustomTimeDilation` 0.0001)
  (`ActorComponent.SetTickableWhenPaused` _timelinemoving true)
  (`TimelineComponent.SetPlayRate` _timelinemoving (* (/ 1.0 (`self.TimeToComplete`)) 10000.0))
  (set `self.StartPoint` (`SceneComponent.K2_GetComponentLocation` (`/Game/_LLTAQ/02_Blueprints/BP_RTSPawn.Cube` (`self.Pawn`))))
  (bind (_direction _newtrack_0) (`Timeline|TimelineMoving`)
    (:`Update`
      (`SceneComponent.K2_SetWorldLocation` (`/Game/_LLTAQ/02_Blueprints/BP_RTSPawn.Cube` (`self.Pawn`)) (`KismetMathLibrary.VLerp` (`self.StartPoint`) (`SceneComponent.K2_GetComponentLocation` (`self.Arrow`)) _newtrack_0) false true))
    (:`Finished`
      (set `self.CustomTimeDilation` 1.0)
      (`self.EnableInput` _returnvalue_2 _returnvalue_2)
      (`/Game/_LLTAQ/02_Blueprints/BP_RTSPawn.DontGoThroughWalls` (`self.Pawn`)))))

(fn `UserConstructionScript`)