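; BP_WinBox is the ant RTS goal object, which triggers victory once enough ants are added.
; On BeginPlay it spawns one randomly placed BP_InteractPoint per required ant and exposes lookups for free points and ants still needed.
; Ant count changes update a sine-bobbing WBP_BlockInfo widget, and additions check the win condition.
; Until won, cursor hover swaps overlay materials, toggles the widget and notifies BP_RTSPlayerController.
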(event `self.ReceiveBeginPlay`
  (bind (_relativelocation_x _relativelocation_y _relativelocation_z) (`KismetMathLibrary.BreakVector` (`SceneComponent.RelativeLocation` (`self.Widget`))))
  (`MeshComponent.SetOverlayMaterial` (`self.StaticMesh`) "/Game/_LLTAQ/07_Materials/M_OutlineBlue.M_OutlineBlue")
  (set `self.Relative Location Z` _relativelocation_z)
  (`self.Update Ant Text`)
  (`self.CreateInteractPoint`))

(event `/Game/_LLTAQ/02_Blueprints/BPI_Interaction.AddAnt`
  (set `self.CurrentAnts` (+ (`self.CurrentAnts`) 1))
  (`self.Update Ant Text`)
  (`SceneComponent.SetVisibility` (`self.Widget`) true false)
  (`self.CheckWinCondition`))

(event `/Game/_LLTAQ/02_Blueprints/BPI_Interaction.RemoveAnt`
  (set `self.CurrentAnts` (- (`self.CurrentAnts`) 1))
  (`self.Update Ant Text`))

(event `self.ReceiveTick`
  (params (DeltaSeconds :type "Float (single-precision)"))
  (`self.MoveWidget` DeltaSeconds))

(event `self.StaticMesh.OnBeginCursorOver`
  (params (TouchedComponent :type "PrimitiveComponent Object Reference"))
  (if (not (`self.HasWon`))
    (`self.StartHover`)))

(event `self.StaticMesh.OnEndCursorOver`
  (params (TouchedComponent :type "PrimitiveComponent Object Reference"))
  (if (not (`self.HasWon`))
    (`self.EndHover`)))

(event `Win`
  (set `self.HasWon` true)
  (`self.EndHover`)
  (`MeshComponent.SetOverlayMaterial` (`self.StaticMesh`) null)
  (`self.OnVictory`))

(fn `CheckWinCondition`
  (if (>= (`self.CurrentAnts`) (`self.RequiredAnt`))
    (`self.Win`)))

(fn `CreateInteractPoint`
  (locals (NewLocalVar :type "Vector Structure" :default (0.0 0.0 0.0)))
  (for _ (range (`self.RequiredAnt`))
    (bind _returnvalue (`|SpawnActorFromClass` "/Game/_LLTAQ/02_Blueprints/BP_InteractPoint.BP_InteractPoint_C" (`SceneComponent.K2_GetComponentToWorld` (`self.HoldPointsRoot`)) "Undefined" "MultiplyWithRoot" null null))
    (`KismetArrayLibrary.Array_Add` (`self.InteractPoints`) _returnvalue)
    (bind _rootcomponent (`Actor.RootComponent` _returnvalue))
    (`SceneComponent.K2_AttachToComponent` _rootcomponent (`self.HoldPointsRoot`) "None" "KeepRelative" "KeepRelative" "KeepRelative" true)
    (`SceneComponent.K2_SetRelativeLocation` _rootcomponent (`KismetMathLibrary.RandomPointInBoundingBox` (0.0 0.0 0.0) (`KismetMathLibrary.Conv_DoubleToVector` (`self.Radius`))) false false)
    (`SceneComponent.K2_SetRelativeRotation` _rootcomponent (`KismetMathLibrary.MakeRotator` 0.0 0.0 (* (`KismetMathLibrary.RandomFloat`) 360.0)) false false)
    (set `/Game/_LLTAQ/02_Blueprints/BP_InteractPoint.Parent` self _returnvalue)))

(fn `EndHover`
  (set `self.Hover` false)
  (`MeshComponent.SetOverlayMaterial` (`self.StaticMesh`) "/Game/_LLTAQ/07_Materials/M_Outline.M_Outline")
  (`SceneComponent.SetVisibility` (`self.Widget`) false false)
  (bind _asbp_rtsplayer_controller (cast `/Game/_LLTAQ/02_Blueprints/BP_RTSPlayerController` (`GameplayStatics.GetPlayerController` 0)))
  (`/Game/_LLTAQ/02_Blueprints/BP_RTSPlayerController.SetHoverActor` _asbp_rtsplayer_controller self false))

(fn `GetAntsNeeded`
  (returns (Value :type Integer))
  (return (- (`self.RequiredAnt`) (`self.CurrentAnts`))))

(fn `GetExitPoint`
  (returns (Arrow :type "ArrowComponent Object Reference"))
  (return null))

(fn `GetFreeInteractPoint`
  (returns (Point :type "/Game/_LLTAQ/02_Blueprints/BP_InteractPoint Object Reference"))
  (for _array_element (`self.InteractPoints`)
    (if (not (`/Game/_LLTAQ/02_Blueprints/BP_InteractPoint.bIsOccupied` _array_element))
      (return _array_element)))
  (return null))

(fn `MoveWidget`
  (params (A :type "Float (double-precision)"))
  (set `self.ElapseTime` (+ A (`self.ElapseTime`)))
  (`SceneComponent.K2_SetRelativeLocation` (`self.Widget`) (`KismetMathLibrary.MakeVector` 0.0 0.0 (+ (* (`self.FloatAmplitude`) (`KismetMathLibrary.Sin` (* (`self.ElapseTime`) (`self.FloatSpeed`)))) (`self.Relative Location Z`))) false false))

(fn `StartHover`
  (set `self.Hover` true)
  (`MeshComponent.SetOverlayMaterial` (`self.StaticMesh`) "/Game/_LLTAQ/07_Materials/M_Hover.M_Hover")
  (`SceneComponent.SetVisibility` (`self.Widget`) true false)
  (bind _asbp_rtsplayer_controller (cast `/Game/_LLTAQ/02_Blueprints/BP_RTSPlayerController` (`GameplayStatics.GetPlayerController` 0)))
  (`/Game/_LLTAQ/02_Blueprints/BP_RTSPlayerController.SetHoverActor` _asbp_rtsplayer_controller self true))

(fn `Update Ant Text`
  (bind _aswbp_block_info (cast `/Game/_LLTAQ/06_UI/WBP_BlockInfo` (`WidgetComponent.GetWidget` (`self.Widget`))))
  (`/Game/_LLTAQ/06_UI/WBP_BlockInfo.UpdateText` _aswbp_block_info (`self.CurrentAnts`) (`self.RequiredAnt`)))

(fn `UserConstructionScript`)