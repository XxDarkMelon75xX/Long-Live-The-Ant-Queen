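; BP_Onsenfou is a selectable unit character that interacts with actors and can be assigned to hold points.
; Selection toggles an outline overlay, and a passed target receives an interface interact message when in range or overlapped.
; When interacted with, it faces the interactor and plays a response animation, also triggered on an Onsenfou interactor.
; Hold-point assignment uses timeline lerps, attaches and disables collision; freeing detaches and moves it to a random reachable point.
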(event `self.StopMovement`
  ; Stop Moving
  (`MovementComponent.StopMovementImmediately` (`self.CharacterMovement`)))

(event `self.UnitSelected`
  ; Reset Animation when Selected
  (`MeshComponent.SetOverlayMaterial` (`self.Mesh`) "/Game/_LLTAQ/07_Materials/M_OutlineBlue.M_OutlineBlue")
  (if (`|EnumInequality` (`SkeletalMeshComponent.GetAnimationMode` (`self.Mesh`)) "AnimationBlueprint")
    (`SkeletalMeshComponent.SetAnimationMode` (`self.Mesh`) "AnimationBlueprint" true)))

(event `self.Interact`
  (params (Interactor :type "Actor Object Reference"))
  ; Interaction Event, activated upon receiving Interact message via Interface. Plays an animation.
  (`|ExecutionSequence`
    (:`then_0`
      (`self.K2_SetActorRotation` (`KismetMathLibrary.FindLookAtRotation` (`self.K2_GetActorLocation`) (`self.K2_GetActorLocation` Interactor)))
      (`self.Interaction Behavior`))
    (:`then_1`
      (bind _asbp_onsenfou (cast `/Game/_LLTAQ/02_Blueprints/BP_Onsenfou` Interactor))
      (`self.Interaction Behavior` _asbp_onsenfou))))

(event `Interaction Behavior`
  (bind _mesh (`self.Mesh`))
  (bind _responseanimation (`self.ResponseAnimation`))
  ; Interaction Event, activated upon receiving Interact message via Interface. Plays an animation.
  (`SkeletalMeshComponent.PlayAnimation` _mesh _responseanimation false)
  (`KismetSystemLibrary.Delay` (`AnimationAsset.GetPlayLength` _responseanimation))
  (`SkeletalMeshComponent.SetAnimationMode` _mesh "AnimationBlueprint" true))

(event `self.MoveCharacterTo`
  (params (Location :type "Vector Structure"))
  (`self.FreeHoldPoint`))

(event `self.PassSelectedActor`
  (params (Actor :type "Actor Object Reference"))
  (bind _output_get (set `self.ActorToInteract` Actor))
  (`self.FreeHoldPoint`)
  (bind _location (message `/Game/_LLTAQ/02_Blueprints/BPI_RTS.GetInteractLocation` _output_get))
  (if (<= (`KismetMathLibrary.Vector_Distance` _location (`SceneComponent.K2_GetComponentLocation` (`self.CapsuleComponent`))) (`self.DistanceToInteract`))
    (message `/Game/_LLTAQ/02_Blueprints/BPI_RTS.Interact` (`self.ActorToInteract`) self)))

(event `self.InteractCollision.OnComponentBeginOverlap`
  (params (OverlappedComponent :type "PrimitiveComponent Object Reference") (OtherActor :type "Actor Object Reference") (OtherComp :type "PrimitiveComponent Object Reference") (OtherBodyIndex :type Integer) (bFromSweep :type Boolean) (SweepResult :type "HitResult Structure (by ref)"))
  (if (== OtherActor (`self.ActorToInteract`))
    (message `/Game/_LLTAQ/02_Blueprints/BPI_RTS.Interact` (`self.ActorToInteract`) self)))

(event `self.UnitDeselected`
  (`MeshComponent.SetOverlayMaterial` (`self.Mesh`) null))

(event `MoveToVector`
  (params (Start :type "Vector Structure") (End :type "Vector Structure"))
  (bind (_direction _t_movetrack) (`Timeline|T_Move` :!via `PlayFromStart`)
    (:`Update`
      (`self.K2_SetActorLocation` (`KismetMathLibrary.VLerp` Start End _t_movetrack) false true))
    (:`Finished`
      (`self.OnMoveFinished`))))

(event `MoveToActor`
  (params (Start :type "Vector Structure") (Actor :type "Actor Object Reference"))
  (bind (_direction _t_movetrack) (`Timeline|Timeline` :!via `PlayFromStart`)
    (:`Update`
      (`self.K2_SetActorLocation` (`KismetMathLibrary.VLerp` Start (`self.K2_GetActorLocation` Actor) _t_movetrack) false true))
    (:`Finished`
      (`self.OnMoveFinished`))))

(fn `AssignHoldPoint`
  (params (HoldPoint :type "/Game/_LLTAQ/02_Blueprints/BP_HoldPoint Object Reference"))
  (`self.FreeHoldPoint`)
  (bind _output_get (set `self.AssignedHoldPoint` HoldPoint))
  (set `self.bIsAssigned` true)
  (`self.StopMovement`)
  (`self.MoveToActor` (`SceneComponent.K2_GetComponentLocation` (`self.CapsuleComponent`)) (`self.AssignedHoldPoint`))
  (`self.K2_AttachToActor` _output_get "None" "KeepWorld" "KeepRelative" "KeepWorld")
  (`PrimitiveComponent.SetCollisionEnabled` (`self.CapsuleComponent`) "NoCollision"))

(fn `DragSelectResult`
  (params (SelectedActors :type "Array of Actor Object Reference (by ref)"))
  (returns (NewParam :type Boolean))
  (return false))

(fn `EnableCollision`
  (`PrimitiveComponent.SetCollisionEnabled` (`self.CapsuleComponent`) "QueryAndPhysics")
  (set `self.bSelectable` true))

(fn `fgezomkgfezkhb`
  (returns (NewParam :type Boolean))
  (return (`self.bSelectable`)))

(fn `FreeHoldPoint`
  (bind _assignedholdpoint (`self.AssignedHoldPoint`))
  (bind _randomlocation (`NavigationSystemV1.K2_GetRandomReachablePointInRadius` (`SceneComponent.K2_GetComponentLocation` (`/Game/_LLTAQ/02_Blueprints/BP_HoldPoint.FreeLocationPoint` (`self.AssignedHoldPoint`))) 300.0 null null))
  (`/Engine/EditorBlueprintResources/StandardMacros.IsValid` _assignedholdpoint
    (:`Is Valid`
      (`self.K2_DetachFromActor` "KeepWorld" "KeepRelative" "KeepWorld")
      (`self.MoveToVector` (`SceneComponent.K2_GetComponentLocation` (`self.CapsuleComponent`)) (`KismetMathLibrary.MakeVector` (.x _randomlocation) (.y _randomlocation) (+ (.z _randomlocation) 40.0)))
      (`/Game/_LLTAQ/02_Blueprints/BP_HoldPoint.FreeUnit` _assignedholdpoint)
      (set `self.bIsAssigned` false)
      (set `self.AssignedHoldPoint` null)
      (add `self.OnMoveFinished` (`|CreateDelegate` :!event `EnableCollision`)))))

(fn `GetInteractLocation`
  (returns (Location :type "Vector Structure"))
  (return (0.0 0.0 0.0)))

(fn `PassSelectedUnits`
  (returns (Actors :type "Array of Actor Object Reference"))
  (return))

(fn `SetMaterial`
  (params (Material :type "MaterialInterface Object Reference"))
  (bind _mesh (`self.Mesh`))
  (`PrimitiveComponent.SetMaterial` _mesh 0 Material)
  (`PrimitiveComponent.SetMaterial` _mesh 1 Material))

(fn `UserConstructionScript`)