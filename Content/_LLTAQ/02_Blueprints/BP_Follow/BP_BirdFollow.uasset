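; Bird character that flies continuously along its facing direction inside a wrapping rectangular area.
; Each tick it overwrites the CharacterMovement velocity with the capsule's horizontal forward vector, normalized and scaled by Speed.
; TeleportX and TeleportY then move it to the opposite edge when it leaves the Min/Max bounds on that axis, preserving height.
; Despite the Follow name, these graphs contain no target tracking or steering.
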(event `self.ReceiveTick`
  (params (DeltaSeconds :type "Float (single-precision)"))
  (bind (_returnvalue_x _returnvalue_y) (`KismetMathLibrary.BreakVector` (`SceneComponent.GetForwardVector` (`self.CapsuleComponent`))))
  (set `MovementComponent.Velocity` (* (`KismetMathLibrary.Normal` (`KismetMathLibrary.MakeVector` _returnvalue_x _returnvalue_y)) (`self.Speed`)) (`self.CharacterMovement`))
  (`self.TeleportX`)
  (`self.TeleportY`))

(fn `TeleportX`
  (bind (_returnvalue_x _returnvalue_y _returnvalue_z) (`KismetMathLibrary.BreakVector` (`self.K2_GetActorLocation`)))
  (bind (_returnvalue_x_2 _returnvalue_y_2 _returnvalue_z_2) (`KismetMathLibrary.BreakVector` (`self.K2_GetActorLocation`)))
  (if (> _returnvalue_x_2 (`self.MaxX`))
    (`self.K2_SetActorLocation` (`KismetMathLibrary.MakeVector` (`self.MinX`) _returnvalue_y_2 _returnvalue_z_2))
    (elif (< _returnvalue_x (`self.MinX`))
      (`self.K2_SetActorLocation` (`KismetMathLibrary.MakeVector` (`self.MaxX`) _returnvalue_y _returnvalue_z)))))

(fn `TeleportY`
  (bind (_returnvalue_x _returnvalue_y _returnvalue_z) (`KismetMathLibrary.BreakVector` (`self.K2_GetActorLocation`)))
  (bind (_returnvalue_x_2 _returnvalue_y_2 _returnvalue_z_2) (`KismetMathLibrary.BreakVector` (`self.K2_GetActorLocation`)))
  (if (> _returnvalue_y (`self.MaxY`))
    (`self.K2_SetActorLocation` (`KismetMathLibrary.MakeVector` _returnvalue_x (`self.MinY`) _returnvalue_z))
    (elif (< _returnvalue_y_2 (`self.MinY`))
      (`self.K2_SetActorLocation` (`KismetMathLibrary.MakeVector` _returnvalue_x_2 (`self.MaxY`) _returnvalue_z_2)))))

(fn `UserConstructionScript`)