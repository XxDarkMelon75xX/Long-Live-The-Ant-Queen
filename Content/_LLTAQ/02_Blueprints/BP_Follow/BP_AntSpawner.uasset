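; BP_AntSpawner spawns a line of BP_AntFollow ants that travel along a spline path.
; On BeginPlay it spawns AntsToSpawn actors at the world origin, giving each the Path spline, TimeToComplete and an evenly spaced BeginOffset fraction along it.
; If the Materials array is not empty, each ant gets a random material from it.
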(event `self.ReceiveBeginPlay`
  (`self.SpawnXAnts` (`self.AntsToSpawn`)))

(fn `SpawnXAnts`
  (params (Value :type Integer))
  (locals (Step :type "Float (double-precision)"))
  (set `local.Step` (/ 1.0 (`KismetMathLibrary.Conv_IntToDouble` Value)))
  (for _index (range 1 (+ Value 1))
    (bind _returnvalue (`|SpawnActorFromClass` "/Game/_LLTAQ/02_Blueprints/BP_Follow/BP_AntFollow.BP_AntFollow_C" (`KismetMathLibrary.MakeTransform` (0.0 0.0 0.0)) "AlwaysSpawn" "MultiplyWithRoot" null null))
    (set `/Game/_LLTAQ/02_Blueprints/BP_FollowSpline.BeginOffset` (* _index (`local.Step`)) _returnvalue)
    (set `/Game/_LLTAQ/02_Blueprints/BP_FollowSpline.MovementSpline` (`self.Path`) _returnvalue)
    (set `/Game/_LLTAQ/02_Blueprints/BP_FollowSpline.TimeToComplete` (`self.Time to Complete`) _returnvalue)
    (if (> (`KismetArrayLibrary.Array_Length` (`self.Materials`)) 0)
      (`/Game/_LLTAQ/02_Blueprints/BP_Follow/BP_AntFollow.SetMaterialCustom` _returnvalue (`KismetArrayLibrary.Array_Random` (`self.Materials`))))))

(fn `UserConstructionScript`)