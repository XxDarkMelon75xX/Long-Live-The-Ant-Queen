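; BP_HoldPoint is a single slot that one unit, apparently an ant, can occupy as part of a parent block.
; AssignUnit stores the unit and marks the point occupied only when it is free, then calls AddAnt on the parent block.
; FreeUnit clears an occupied point and calls RemoveAnt, so the block is notified of each change in occupancy.
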(fn `AssignUnit`
  (params (Unit :type "/Game/_LLTAQ/02_Blueprints/BP_RTSUnit Object Reference"))
  (if (not (`self.bIsOccupied`))
    (set `self.CurrentUnit` Unit)
    (set `self.bIsOccupied` true)
    (`/Game/_LLTAQ/02_Blueprints/BP_Block.AddAnt` (`self.ParentBlock`))))

(fn `FreeUnit`
  (if (`self.bIsOccupied`)
    (set `self.CurrentUnit` null)
    (set `self.bIsOccupied` false)
    (`/Game/_LLTAQ/02_Blueprints/BP_Block.RemoveAnt` (`self.ParentBlock`))))

(fn `UserConstructionScript`)