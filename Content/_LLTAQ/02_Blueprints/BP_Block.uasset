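; Block that RTS units (ants) surround and, once enough hold it, carries along a spline.
; BeginPlay spawns RequiredAnts hold point actors in a ring, previewed with billboards by the construction script.
; Interact assigns a unit not yet assigned to the first free hold point.
; CheckMovable calls Move when all points are occupied, playing a one-shot timeline along the spline; an older straight-line move is left unconnected.
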(event `self.ReceiveBeginPlay`
  (`self.CreateHoldPoints`)
  (`TimelineComponent.SetPlayRate` (`self.Timeline_0`) (`self.PlayRate`)))

(event `/Game/_LLTAQ/02_Blueprints/BPI_RTS.Interact`
  (params (Interactor :type "Actor Object Reference"))
  (bind _asbp_rtsunit (cast `/Game/_LLTAQ/02_Blueprints/BP_RTSUnit` Interactor))
  (bind _here (`self.IsAssigned` _asbp_rtsunit))
  (if (not _here)
    (bind _holdpoint (`self.GetFreeHoldPoint`))
    (`/Engine/EditorBlueprintResources/StandardMacros.IsValid` _holdpoint
      (:`Is Valid`
        (`/Game/_LLTAQ/02_Blueprints/BP_HoldPoint.AssignUnit` _holdpoint _asbp_rtsunit)
        (`/Game/_LLTAQ/02_Blueprints/BP_RTSUnit.AssignHoldPoint` _asbp_rtsunit _holdpoint)))))

(event `Move`
  (bind _spline (`/Game/_LLTAQ/02_Blueprints/BP_Path.Spline` (`self.Spline`)))
  (if (not (`self.HasMoved`))
    (set `self.HasMoved` true)
    (`TimelineComponent.SetPlayRate` (`self.T_Move`) (/ 1.0 (`self.TimeToComplete`)))
    (bind (_direction _t_move_track) (`Timeline|T_Move` :!via `PlayFromStart`)
      (:`Update`
        (bind _returnvalue (`KismetMathLibrary.Lerp` 0.0 (`SplineComponent.GetSplineLength` _spline) _t_move_track))
        (`self.K2_SetActorLocationAndRotation` (`SplineComponent.GetLocationAtDistanceAlongSpline` _spline _returnvalue "World") (`SplineComponent.GetRotationAtDistanceAlongSpline` _spline _returnvalue "World") false true)))))

(fn `CheckMovable`
  (for _array_element (`self.HoldPoints`)
    (if (not (`/Game/_LLTAQ/02_Blueprints/BP_HoldPoint.bIsOccupied` _array_element))
      (set `self.bMovable` false)
      (return)))
  (set `self.bMovable` true)
  (`self.Move`))

(fn `CreateHoldPoints`
  (locals (AngleStep :type "Float (double-precision)" :default 0.0) (Angle :type "Float (double-precision)") (X :type "Float (double-precision)") (Y :type "Float (double-precision)") (Z :type "Float (double-precision)" :default 0.0))
  (set `local.AngleStep` (/ 360.0 (`KismetMathLibrary.Conv_IntToDouble` (`self.RequiredAnts`))))
  (for _index (range (`self.RequiredAnts`))
    (set `local.Angle` (+ (* _index (`local.AngleStep`)) (`self.SurroundRotationOffset`)))
    (set `local.X` (* (`KismetMathLibrary.DegCos` (`local.Angle`)) (`self.SurroundRadius`)))
    (set `local.Y` (* (`KismetMathLibrary.DegSin` (`local.Angle`)) (`self.SurroundRadius`)))
    (set `local.Z` (`self.SurroundHeightOffset`))
    (bind _returnvalue (`|SpawnActorFromClass` "/Game/_LLTAQ/02_Blueprints/BP_HoldPoint.BP_HoldPoint_C" (`SceneComponent.K2_GetComponentToWorld` (`self.HoldPointsRoot`)) "Undefined" "MultiplyWithRoot" null null))
    (`KismetArrayLibrary.Array_Add` (`self.HoldPoints`) _returnvalue)
    (bind _rootcomponent (`Actor.RootComponent` _returnvalue))
    (`SceneComponent.K2_AttachToComponent` _rootcomponent (`self.HoldPointsRoot`) "None" "KeepRelative" "KeepRelative" "KeepRelative" true)
    (`SceneComponent.K2_SetRelativeLocation` _rootcomponent (`KismetMathLibrary.MakeVector` (`local.X`) (`local.Y`) (`local.Z`)) false false)
    (set `/Game/_LLTAQ/02_Blueprints/BP_HoldPoint.ParentBlock` self _returnvalue)
    (set `/Game/_LLTAQ/02_Blueprints/BP_HoldPoint.FreeLocationPoint` (`self.InteractLocation`) _returnvalue)))

(fn `DragSelectResult`
  (params (SelectedActors :type "Array of Actor Object Reference (by ref)"))
  (returns (NewParam :type Boolean))
  (return false))

(fn `GetFreeHoldPoint`
  (returns (HoldPoint :type "/Game/_LLTAQ/02_Blueprints/BP_HoldPoint Object Reference"))
  (for _array_element (`self.HoldPoints`)
    (if (not (`/Game/_LLTAQ/02_Blueprints/BP_HoldPoint.bIsOccupied` _array_element))
      (return _array_element)))
  (return null))

(fn `GetInteractLocation`
  (returns (Location :type "Vector Structure"))
  (return (`SceneComponent.K2_GetComponentLocation` (`self.InteractLocation`))))

(fn `IsAssigned`
  (params (Unit :type "/Game/_LLTAQ/02_Blueprints/BP_RTSUnit Object Reference"))
  (returns (Here :type Boolean))
  (for _array_element (`self.HoldPoints`)
    (if (== (`/Game/_LLTAQ/02_Blueprints/BP_HoldPoint.CurrentUnit` _array_element) Unit)
      (return true)))
  (return false))

(fn `PassSelectedUnits`
  (returns (Actors :type "Array of Actor Object Reference"))
  (return))

(fn `UserConstructionScript`
  (locals (AngleStep :type "Float (double-precision)") (Angle :type "Float (double-precision)") (X :type "Float (double-precision)") (Y :type "Float (double-precision)") (Z :type "Float (double-precision)"))
  (set `local.AngleStep` (/ 360.0 (`KismetMathLibrary.Conv_IntToDouble` (`self.RequiredAnts`))))
  (for _index (range (`self.RequiredAnts`))
    (set `local.Angle` (+ (* _index (`local.AngleStep`)) (`self.SurroundRotationOffset`)))
    (set `local.X` (* (`KismetMathLibrary.DegCos` (`local.Angle`)) (`self.SurroundRadius`)))
    (set `local.Y` (* (`KismetMathLibrary.DegSin` (`local.Angle`)) (`self.SurroundRadius`)))
    (set `local.Z` (`self.SurroundHeightOffset`))
    (bind _returnvalue (`AddComponent|NODE_AddBillboardComponent-0`))
    (`SceneComponent.K2_SetRelativeLocation` _returnvalue (`KismetMathLibrary.MakeVector` (`local.X`) (`local.Y`) (`local.Z`)) false false)))