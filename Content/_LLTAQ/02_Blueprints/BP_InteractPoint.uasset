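; BP_InteractPoint is a single-occupancy slot that one unit at a time can claim, apparently for ants interacting with a parent object.
; AssignUnit stores the unit and marks the point occupied only if it is free, then calls AddAntMessage on its Parent.
; FreeUnit clears an occupied point and calls RemoveAntMessage, so the Parent is notified only when occupancy actually changes.
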(fn `AssignUnit`
  (params (Unit :type "/Game/_LLTAQ/02_Blueprints/BP_RTSUnit Object Reference"))
  (if (not (`self.bIsOccupied`))
    (set `self.CurrentUnit` Unit)
    (set `self.bIsOccupied` true)
    (message `/Game/_LLTAQ/02_Blueprints/BPI_Interaction.AddAnt` (`self.Parent`))))

(fn `FreeUnit`
  (if (`self.bIsOccupied`)
    (set `self.CurrentUnit` null)
    (set `self.bIsOccupied` false)
    (message `/Game/_LLTAQ/02_Blueprints/BPI_Interaction.RemoveAnt` (`self.Parent`))))

(fn `UserConstructionScript`)