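; BP_ObjectRenderer is a one-shot trigger volume that shows or hides a referenced actor when an RTS unit enters it.
; A box overlap filters for BP_RTSUnit, then the Activate flag selects Enable or Disable to set the target Actor's hidden-in-game state.
; Both events then call DestroyActor, so the trigger fires only once.
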(event `self.Box.OnComponentBeginOverlap`
  (params (OverlappedComponent :type "PrimitiveComponent Object Reference") (OtherActor :type "Actor Object Reference") (OtherComp :type "PrimitiveComponent Object Reference") (OtherBodyIndex :type Integer) (bFromSweep :type Boolean) (SweepResult :type "HitResult Structure (by ref)"))
  (cast `/Game/_LLTAQ/02_Blueprints/BP_RTSUnit` OtherActor)
  (if (`self.Activate`)
    (`self.Enable`)
    (else
      (`self.Disable`))))

(event `Enable`
  (`self.SetActorHiddenInGame` (`self.Actor`) false)
  (`self.K2_DestroyActor`))

(event `Disable`
  (`self.SetActorHiddenInGame` (`self.Actor`) true)
  (`self.K2_DestroyActor`))

(fn `UserConstructionScript`)