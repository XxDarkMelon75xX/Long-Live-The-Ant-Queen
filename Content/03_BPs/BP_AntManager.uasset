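; BP_AntManager tracks the level's ant characters and dispatches or recalls them.
; On BeginPlay it gathers all BP_AntCharacters and picks a random available leader with movement avoidance disabled.
; SendAnts assigns random available ants to a BP_Clickable's unoccupied points, moving them to the unavailable list.
; Recall functions return all dispatched ants or those from the last clicked object's points, then reselect the leader.
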(event `self.ReceiveBeginPlay`
  (`self.GetAnts`)
  (`self.ChooseRandomLeader`))

(fn `ChooseRandomLeader`
  (bind _availableants (`self.AvailableAnts`))
  (bind _currentleader (`self.CurrentLeader`))
  (`/Engine/EditorBlueprintResources/StandardMacros.IsValid` _currentleader
    (:`Is Valid`
      (`CharacterMovementComponent.SetAvoidanceEnabled` (`Character.CharacterMovement` _currentleader) true))
    (:`Is Not Valid`
      _))
  (if (> (`KismetArrayLibrary.Array_Length` _availableants) 0)
    (bind _output_get (set `self.CurrentLeader` (`KismetArrayLibrary.Array_Random` _availableants)))
    (`CharacterMovementComponent.SetAvoidanceEnabled` (`Character.CharacterMovement` _output_get) false)))

(fn `GetAnts`
  (bind _outactors (`GameplayStatics.GetAllActorsOfClass` "/Game/03_BPs/BP_AntCharacter.BP_AntCharacter_C"))
  (bind _output_get (set `self.Ants` _outactors))
  (set `self.AvailableAnts` _output_get))

(fn `RecallAllAnts`
  (`self.RecallSetAnts` (`self.UnavailableAnts`)))

(fn `RecallLastObjectAnts`
  (locals (Ants :type "Array of /Game/03_BPs/BP_AntCharacter Object Reference"))
  (bind _asbp_clickable (cast `/Game/03_BPs/BP_Clickable` (`self.LastActorClicked`)))
  (bind _points (`/Game/03_BPs/BP_Clickable.GetAllPoints` _asbp_clickable))
  (for _array_element _points
    (if (`/Game/03_BPs/Component/BP_FollowerLocationComponent.IsOccupied` _array_element)
      _
      (else
        _))
    (`KismetArrayLibrary.Array_Add` (`local.Ants`) (`/Game/03_BPs/Component/BP_FollowerLocationComponent.Ant` _array_element)))
  (set `self.LastActorClicked` null)
  (`self.RecallSetAnts` (`local.Ants`)))

(fn `RecallSetAnts`
  (params (Ants :type "Array of /Game/03_BPs/BP_AntCharacter Object Reference"))
  (locals (AntsToClear :type "Array of /Game/03_BPs/BP_AntCharacter Object Reference"))
  (`KismetSystemLibrary.PrintString` (`KismetStringLibrary.Conv_IntToString` (`KismetArrayLibrary.Array_Length` Ants)))
  (for _array_element Ants
    (`/Game/03_BPs/BP_AntCharacter.Recall` _array_element)
    (`KismetArrayLibrary.Array_Add` (`self.AvailableAnts`) _array_element)
    (`KismetArrayLibrary.Array_Add` (`local.AntsToClear`) _array_element))
  (for _array_element_2 (`local.AntsToClear`)
    (`KismetArrayLibrary.Array_RemoveItem` (`self.UnavailableAnts`) _array_element_2))
  (`self.ChooseRandomLeader`))

(fn `RegisterAnt`
  (params (NewAnt :type "/Game/03_BPs/BP_AntCharacter Object Reference"))
  (if (not (`KismetArrayLibrary.Array_Contains` (`self.Ants`) NewAnt))
    (`KismetArrayLibrary.Array_Add` (`self.Ants`) NewAnt)))

(fn `SendAnts`
  (params (Actor :type "Actor Object Reference"))
  (bind _asbp_clickable (cast `/Game/03_BPs/BP_Clickable` Actor)
    (:`then`
      (set `self.LastActorClicked` Actor)
      (bind _points (`/Game/03_BPs/BP_Clickable.GetUnoccupiedPoints` _asbp_clickable))
      (for _array_element _points
        (bind _output_get (set `self.CurrAnt` (`KismetArrayLibrary.Array_Random` (`self.AvailableAnts`))))
        (`/Game/03_BPs/BP_AntCharacter.NewFollowOrder` _output_get _array_element)
        (`KismetArrayLibrary.Array_RemoveItem` (`self.AvailableAnts`) (`self.CurrAnt`))
        (`KismetArrayLibrary.Array_Add` (`self.UnavailableAnts`) (`self.CurrAnt`))
        (`self.ChooseRandomLeader`)))
    (:`CastFailed`
      (`KismetSystemLibrary.PrintString` "NotClickable"))))

(fn `UnregisterAnt`
  (params (AntToRemove :type "/Game/03_BPs/BP_AntCharacter Object Reference"))
  (`KismetArrayLibrary.Array_RemoveItem` (`self.Ants`) AntToRemove)
  (if (== AntToRemove (`self.CurrentLeader`))
    (`self.ChooseRandomLeader`)))

(fn `UserConstructionScript`)