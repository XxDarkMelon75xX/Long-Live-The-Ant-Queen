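; BP_AntPawn is an ant pawn that follows BP_AntPlayer's FollowPoint while keeping apart from other ants.
; Two looping timers with start-delay variance drive it, one for following and one for separation.
; The follow check issues AIMoveTo when the ant strays too far from that point.
; Separation overlaps a sphere for nearby ants, averages distance-weighted repulsion vectors, and applies the clamped result as physics force on the Cube.
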(event `self.ReceiveBeginPlay`
  (bind _returnvalue (`GameplayStatics.GetActorOfClass` "/Game/03_BPs/BP_AntPlayer.BP_AntPlayer_C"))
  (set `self.AntPlayer` _returnvalue)
  (`KismetSystemLibrary.K2_SetTimerDelegate` (delegate `Repulsion`) 0.1 true true 0.0 0.15)
  (`KismetSystemLibrary.K2_SetTimerDelegate` (delegate `DistanceCheck`) 0.2 true true 0.0 0.15))

(event `FollowPlayer`
  (`|AIMoveTo` self (`SceneComponent.K2_GetComponentLocation` (`/Game/03_BPs/BP_AntPlayer.FollowPoint` (`self.AntPlayer`))) null 200.0))

(event `Repulsion`
  (`self.ApplyRepulsion`))

(event `DistanceCheck`
  (if (not (<= (`KismetMathLibrary.Vector_Distance` (`SceneComponent.K2_GetComponentLocation` (`/Game/03_BPs/BP_AntPlayer.FollowPoint` (`self.AntPlayer`))) (`self.K2_GetActorLocation`)) 1000.0))
    (`self.FollowPlayer`)))

(fn `ApplyRepulsion`
  (bind _outactors (`KismetSystemLibrary.SphereOverlapActors` (`self.K2_GetActorLocation`) (`self.MaxDistance`) (`|MakeArray` "ObjectTypeQuery3" "ObjectTypeQuery4" :!type "EObjectTypeQuery Enum") "BP_AntPawn_C"))
  (`KismetArrayLibrary.Array_RemoveItem` _outactors self)
  (bind _closestactors (`self.GetClosestActors` _outactors))
  (bind _force (`self.GetRepulsiveVector` _closestactors))
  (`PrimitiveComponent.AddForce` (`self.Cube`) _force "None" false))

(fn `GetClosestActors`
  (params (Actors :type "Array of Actor Object Reference"))
  (returns (ClosestActors :type "Array of /Game/05_Struct/S_ActorDistance Structure"))
  (locals (ActorDistance :type "Array of /Game/05_Struct/S_ActorDistance Structure"))
  (bind _returnvalue (`self.K2_GetActorLocation`))
  (for _array_element Actors
    (bind _returnvalue_2 (`self.K2_GetActorLocation` _array_element))
    (`KismetArrayLibrary.Array_AddUnique` (`local.ActorDistance`) (make `/Game/05_Struct/S_ActorDistance` (`KismetMathLibrary.Vector_Distance` _returnvalue_2 _returnvalue) _array_element (`KismetMathLibrary.Normal` (- _returnvalue_2 _returnvalue)))))
  (return (`local.ActorDistance`)))

(fn `GetRepulsiveVector`
  (params (Actors :type "Array of /Game/05_Struct/S_ActorDistance Structure"))
  (returns (Force :type "Vector Structure"))
  (locals (Sum :type "Vector Structure") (Weight :type "Float (double-precision)") (TotalForce :type "Vector Structure"))
  (bind _returnvalue (`KismetArrayLibrary.Array_Length` Actors))
  (if (== _returnvalue 0)
    (return (0.0 0.0 0.0))
    (else
      (for _array_element Actors
        (bind (_distance _actor _direction) (break `/Game/05_Struct/S_ActorDistance` _array_element))
        (bind _output_get (set `local.Weight` (- 1.0 (`KismetMathLibrary.FClamp` (/ (- _distance (`self.MinDistance`)) (- (`self.MaxDistance`) (`self.MinDistance`)))))))
        (set `local.TotalForce` (+ (`local.TotalForce`) (* _output_get (`self.BaseStrength`) _direction -1.0))))
      (return (`KismetMathLibrary.ClampVectorSize` (/ (`local.TotalForce`) _returnvalue) 0.0 2000.0)))))

(fn `UserConstructionScript`)