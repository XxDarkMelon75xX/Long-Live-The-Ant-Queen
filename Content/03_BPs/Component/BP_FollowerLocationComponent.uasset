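; BP_FollowerLocationComponent is a component that tracks one follower slot that an ant can occupy.
; SetAnt stores the ant and marks the slot occupied, or clears occupancy and the in-position state when the ant is invalid.
; SetInPosition fires the OnInPosition dispatcher only when the in-position flag changes.
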(fn `SetAnt`
  (params (Ant :type "/Game/03_BPs/BP_AntCharacter Object Reference"))
  (bind _output_get (set `self.Ant` Ant))
  (`/Engine/EditorBlueprintResources/StandardMacros.IsValid` _output_get
    (:`Is Valid`
      (set `self.IsOccupied` true))
    (:`Is Not Valid`
      (`self.SetInPosition` false)
      (set `self.IsOccupied` false))))

(fn `SetInPosition`
  (params (b :type Boolean))
  (if (!= b (`self.IsInPosition`))
    (set `self.IsInPosition` b)
    (`self.OnInPosition`)))