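; BP_SplinePath is a spline actor that lays a trail of disc decals along a path, built entirely in the construction script.
; It first line-traces vertically around each spline point within DecalSnapThreshold and moves points to hits, writing the world-space hit as a local location.
; It then adds DiscMaterial decals at fixed distance intervals, all pitched from the spline's starting rotation.
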(fn `UserConstructionScript`
  (`|ExecutionSequence`
    (:`then_0`
      (for _index (range (`SplineComponent.GetNumberOfSplinePoints` (`self.Spline`)))
        (bind (_returnvalue_x _returnvalue_y _returnvalue_z) (`KismetMathLibrary.BreakVector` (`SplineComponent.GetLocationAtSplinePoint` (`self.Spline`) _index "World")))
        (bind (_returnvalue_x_2 _returnvalue_y_2 _returnvalue_z_2) (`KismetMathLibrary.BreakVector` (`SplineComponent.GetLocationAtSplinePoint` (`self.Spline`) _index "World")))
        (bind (_outhit _returnvalue) (`KismetSystemLibrary.LineTraceSingle` :`Start` (`KismetMathLibrary.MakeVector` _returnvalue_x _returnvalue_y (+ _returnvalue_z (`self.DecalSnapThreshold`))) :`End` (`KismetMathLibrary.MakeVector` _returnvalue_x_2 _returnvalue_y_2 (- _returnvalue_z_2 (`self.DecalSnapThreshold`))) :`TraceChannel` "TraceTypeQuery1" :`DrawDebugType` "ForDuration"))
        (if _returnvalue
          (`SplineComponent.SetLocationAtSplinePoint` (`self.Spline`) _index (`.Location` (`GameplayStatics.BreakHitResult` _outhit)) "Local" true))))
    (:`then_1`
      (for _index_2 (range (+ (`KismetMathLibrary.FTrunc` (/ (`SplineComponent.GetSplineLength` (`self.Spline`)) 512.0)) 1))
        (bind _returnvalue_2 (`AddComponent|NODE_AddDecalComponent-0`))
        (bind (_returnvalue_roll _returnvalue_pitch _returnvalue_yaw) (`KismetMathLibrary.BreakRotator` (`SplineComponent.GetRotationAtDistanceAlongSpline` (`self.Spline`) (* _index_2 0.0) "World")))
        (`SceneComponent.K2_SetWorldLocationAndRotation` _returnvalue_2 (`SplineComponent.GetLocationAtDistanceAlongSpline` (`self.Spline`) (* _index_2 512.0) "World") (`KismetMathLibrary.MakeRotator` _returnvalue_roll (- _returnvalue_pitch 90.0) _returnvalue_yaw) false false)
        (`DecalComponent.SetDecalMaterial` _returnvalue_2 "/Engine/VREditor/UI/DiscMaterial.DiscMaterial")))))