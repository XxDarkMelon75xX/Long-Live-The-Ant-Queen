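; BP_Ant is an ant actor whose skeletal mesh, animation and material are configured at construction time.
; When ToggleConstruction is on, the Construction Script looks up Type in a Map and applies that entry's mesh.
; The entry's Class (Ant, Attack or Kami) selects the matching Anim Blueprint, then Material is applied to the first slot.
; The event graph holds no runtime logic.
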(fn `UserConstructionScript`
  (bind (_value _returnvalue) (`BlueprintMapLibrary.Map_Find` (`self.Map`) (`self.Type`)))
  (if (`self.bToggleConstruction`)
    (if _returnvalue
      (set `SkeletalMeshComponent.SkeletalMeshAsset` (break `/Game/05_Struct/S_AntModelAnim` _value) (`self.Mesh`))
      (switch `/Game/03_BPs/Enum_AntClass` (`.Class_8_81B801FA421301A53E644DB12B47AF3E` (break `/Game/05_Struct/S_AntModelAnim` _value))
        (:`NewEnumerator0`
          (`SkeletalMeshComponent.SetAnimInstanceClass` (`self.Mesh`) "/Game/06_Ant/BA_Ant.BA_Ant_C"))
        (:`NewEnumerator1`
          (`SkeletalMeshComponent.SetAnimInstanceClass` (`self.Mesh`) "/Game/06_Ant/Ant_02/BA_Ant02.BA_Ant02_C"))
        (:`NewEnumerator3`
          (`SkeletalMeshComponent.SetAnimInstanceClass` (`self.Mesh`) "/Game/06_Ant/Ant_Kami/BA_AntKami.BA_AntKami_C")))
      (`PrimitiveComponent.SetMaterial` (`self.Mesh`) 0 (`self.Material`)))))