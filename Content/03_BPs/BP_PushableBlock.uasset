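; BP_PushableBlock is a block pawn that needs a set number of ants in position before it can move.
; On BeginPlay it spawns follower-location components evenly around a circle, each with a debug sphere, and binds their in-position and leaving events.
; A readiness check requires every point to be in position, gating click-driven AI movement.
; It also exposes its points, the count of unoccupied slots and an immediate stop.
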(event `self.ReceiveBeginPlay`
  (`self.CreateFollowPoints`))

(event `/Game/03_BPs/BP_Clickable.ClickAt`
  (params (Location :type "Vector Structure"))
  (if (`self.bIsReady`)
    (`|AIMoveTo` self Location null)))

(event `/Game/03_BPs/BP_Clickable.Stop`
  (`MovementComponent.StopMovementImmediately` (`self.CharacterMovement`)))

(fn `CheckIfReady`
  (for _array_element (`self.Points`)
    (if (not (`/Game/03_BPs/Component/BP_FollowerLocationComponent.IsInPosition` _array_element))
      (set `self.bIsReady` false)
      (return)))
  (set `self.bIsReady` true)
  (`KismetSystemLibrary.PrintString` "BlockReady"))

(fn `CreateDebugVisual`
  (params (InputPin :type "/Game/03_BPs/Component/BP_FollowerLocationComponent Object Reference"))
  (bind _returnvalue (`AddComponent|NODE_AddStaticMeshComponent-0`))
  (`SceneComponent.K2_AttachToComponent` _returnvalue InputPin "None" "KeepRelative" "KeepRelative" "KeepRelative" true)
  (`StaticMeshComponent.SetStaticMesh` _returnvalue "/Engine/EditorMeshes/EditorSphere.EditorSphere")
  (`SceneComponent.SetWorldScale3D` _returnvalue (0.2 0.2 0.2))
  (`PrimitiveComponent.SetCollisionEnabled` _returnvalue "NoCollision"))

(fn `CreateFollowPoints`
  (for _index (range 1 (+ (`self.AntRequired`) 1))
    (bind _returnvalue (* _index (/ (* 2.0 (`KismetMathLibrary.GetPI`)) (`self.AntRequired`))))
    (bind _returnvalue_2 (`AddComponent|NODE_AddBP_FollowerLocationComponent-0` :`RelativeTransform` (`KismetMathLibrary.Conv_VectorToTransform` (* (`KismetMathLibrary.MakeVector` (`KismetMathLibrary.Cos` _returnvalue) (`KismetMathLibrary.Sin` _returnvalue)) (`self.SpacingRadius`)))))
    (add `/Game/03_BPs/Component/BP_FollowerLocationComponent.OnInPosition` _returnvalue_2 (`|CreateDelegate` :!event `CheckIfReady`))
    (add `/Game/03_BPs/Component/BP_FollowerLocationComponent.OnAntLeaving` _returnvalue_2 (`|CreateDelegate` :!event `Stop`))
    (`KismetArrayLibrary.Array_Add` (`self.Points`) _returnvalue_2)
    (`self.CreateDebugVisual` _returnvalue_2)))

(fn `GetAllPoints`
  (returns (Points :type "Array of /Game/03_BPs/Component/BP_FollowerLocationComponent Object Reference"))
  (return (`self.Points`)))

(fn `GetAntsNeeded`
  (returns (AntsNeeded :type Integer))
  (locals (Ants :type Integer :default 0))
  (for _array_element (`self.Points`)
    (if (not (`/Game/03_BPs/Component/BP_FollowerLocationComponent.IsOccupied` _array_element))
      (`/Engine/EditorBlueprintResources/StandardMacros.IncrementInt` (`local.Ants`))))
  (return (`local.Ants`)))

(fn `UserConstructionScript`)