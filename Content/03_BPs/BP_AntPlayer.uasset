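; Player-controlled ant that AI-moves to locations left-clicked through BP_PlayerCamera and toggles its follow mode on right-click, broadcasting the change.
; It supplies follower slots, returning an existing location component flagged IsOccupied or adding one in a column-and-row grid offset from FollowPoint.
; Health, healing and damage calls forward to a damage system component, whose death, block and response events, like AnyDamage, only print debug strings.
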(event `self.ReceiveBeginPlay`
  (bind _asbp_player_camera (cast `/Game/03_BPs/BP_PlayerCamera` (`GameplayStatics.GetPlayerPawn` 0)))
  (add `/Game/03_BPs/BP_PlayerCamera.OnLeftClick` _asbp_player_camera (delegate `Handle_OnLeftClick`))
  (add `/Game/03_BPs/BP_PlayerCamera.OnRightClick` _asbp_player_camera (delegate `Handle_OnRightClick`)))

(event `Handle_OnLeftClick`
  (params (Location :type "Vector Structure"))
  (`|AIMoveTo` self Location null))

(event `Handle_OnRightClick`
  (`self.CycleFollowEnum`)
  (`self.OnRightClick` (`self.FollowMode`)))

(event `self.ReceiveAnyDamage`
  (params (Damage :type "Float (single-precision)") (DamageType :type "DamageType Object Reference") (InstigatedBy :type "Controller Object Reference") (DamageCauser :type "Actor Object Reference"))
  (`KismetSystemLibrary.PrintString` (`KismetStringLibrary.Concat_StrStr` (`KismetSystemLibrary.GetDisplayName` self) "Damaged By" (`KismetSystemLibrary.GetDisplayName` DamageCauser)) true true (struct :`R` 1.0 :`G` 0.005257 :`A` 1.0)))

(event `Death`
  (`KismetSystemLibrary.PrintString` "DEAD"))

(event `Blocked`
  (params (CanBeParried :type Boolean))
  (`KismetSystemLibrary.PrintString` "BLOCKED"))

(event `DamageResponse`
  (params (DamageResponse :type "/Game/06_DamageSystem/Enum_DamageResponse Enum" :default "NewEnumerator0"))
  (`KismetSystemLibrary.PrintString` (`|GetEnumeratorNameAsString` DamageResponse)))

(fn `CalculateNewFollowerPosition`
  (returns (Transform :type "Transform Structure"))
  (bind _returnvalue (`SceneComponent.GetRelativeTransform` (`self.FollowPoint`)))
  (return (`KismetMathLibrary.MakeTransform` (`KismetMathLibrary.MakeVector` (- (.x (.location _returnvalue)) (* (- (/ (- (`self.FollowerLocationCount`) (mod (`self.FollowerLocationCount`) (`self.ColumnCount`))) (`self.ColumnCount`)) 1) (`self.RowSpacing`))) (+ (- (.y (.location _returnvalue)) (/ (* (- (`self.ColumnCount`) 1) (`self.ColumnSpacing`)) 2.0)) (* (mod (`self.FollowerLocationCount`) (`self.ColumnCount`)) (`self.ColumnSpacing`))) (.z (.location _returnvalue))) (.rotation _returnvalue) (.scale _returnvalue))))

(fn `CycleFollowEnum`
  (set `self.FollowMode` (cast `/Game/03_BPs/Enum_FollowMode` (mod (+ (`self.FollowMode`) 1) 2))))

(fn `GetCurrentHealth`
  (returns (Health :type "Float (double-precision)"))
  (return (`/Game/06_DamageSystem/BPC_DamageSystemComp.Health` (`self.BPC_DamageSystemComp`))))

(fn `GetMaxHealth`
  (returns (MaxHealth :type "Float (double-precision)"))
  (return (`/Game/06_DamageSystem/BPC_DamageSystemComp.MaxHealth` (`self.BPC_DamageSystemComp`))))

(fn `GetNewFollowerLocation`
  (returns (Location :type "/Game/03_BPs/Component/BP_FollowerLocationComponent Object Reference"))
  (for _array_element (`self.K2_GetComponentsByClass` "/Game/03_BPs/Component/BP_FollowerLocationComponent.BP_FollowerLocationComponent_C")
    (if (`/Game/03_BPs/Component/BP_FollowerLocationComponent.IsOccupied` _array_element)
      (return _array_element)))
  (bind _transform (`self.CalculateNewFollowerPosition`))
  (bind _returnvalue (`|AddComponentByClass` "/Game/03_BPs/Component/BP_FollowerLocationComponent.BP_FollowerLocationComponent_C" false _transform))
  (`/Engine/EditorBlueprintResources/StandardMacros.IncrementInt` (`self.FollowerLocationCount`)
    (:`  `
      (return _returnvalue))))

(fn `Heal`
  (params (Amount :type "Float (double-precision)"))
  (returns (NewHealth :type "Float (double-precision)"))
  (bind _newhealth (`/Game/06_DamageSystem/BPC_DamageSystemComp.Heal` (`self.BPC_DamageSystemComp`) Amount))
  (return _newhealth))

(fn `TakeDamage`
  (params (DamageInfo :type "/Game/06_DamageSystem/S_DamageInfo Structure"))
  (returns (WasDamaged :type Boolean))
  (bind _wasdamaged (`/Game/06_DamageSystem/BPC_DamageSystemComp.TakeDamage` (`self.BPC_DamageSystemComp`) DamageInfo))
  (return _wasdamaged))

(fn `UserConstructionScript`
  (bind _bpc_damagesystemcomp (`self.BPC_DamageSystemComp`))
  (add `/Game/06_DamageSystem/BPC_DamageSystemComp.OnDeath` _bpc_damagesystemcomp (`|CreateDelegate` :!event `Death`))
  (add `/Game/06_DamageSystem/BPC_DamageSystemComp.OnBlocked` _bpc_damagesystemcomp (`|CreateDelegate` :!event `Blocked`))
  (add `/Game/06_DamageSystem/BPC_DamageSystemComp.OnDamageResponse` _bpc_damagesystemcomp (`|CreateDelegate` :!event `DamageResponse`)))