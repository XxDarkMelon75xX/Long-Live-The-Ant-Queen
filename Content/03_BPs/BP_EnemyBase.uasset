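; BP_EnemyBase is a base enemy pawn, currently mostly a scaffold for health and damage handling.
; Death, Blocked and DamageResponse events only print debug text, while UpdateSpeed sets the FloatingPawnMovement max speed.
; TakeDamage and Heal are empty, and health and death queries return fixed defaults.
; ApplyDamageToPlayer is also empty, with its forward sphere-trace melee hit left disconnected.
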(event `Death`
  (`KismetSystemLibrary.PrintString` "DEAD" true true (struct :`R` 1.0 :`B` 0.003035 :`A` 1.0)))

(event `Blocked`
  (params (CanBeParried :type Boolean))
  (`KismetSystemLibrary.PrintString` "BLOCKED" true true (struct :`R` 1.0 :`B` 0.003035 :`A` 1.0)))

(event `DamageResponse`
  (params (DamageResponse :type "/Game/06_DamageSystem/Enum_DamageResponse Enum" :default "NewEnumerator0"))
  (`KismetSystemLibrary.PrintString` (`|GetEnumeratorNameAsString` DamageResponse) true true (struct :`R` 1.0 :`B` 0.003035 :`A` 1.0)))

(fn `ApplyDamageToPlayer`)

(fn `GetCurrentHealth`
  (returns (Health :type "Float (double-precision)"))
  (return 0.0))

(fn `GetMaxHealth`
  (returns (MaxHealth :type "Float (double-precision)"))
  (return 0.0))

(fn `Heal`
  (params (Amount :type "Float (double-precision)" :default 0.0))
  (returns (NewHealth :type "Float (double-precision)")))

(fn `IsDead`
  (returns (ReturnValue :type Boolean))
  (return false))

(fn `TakeDamage`
  (params (DamageInfo :type "/Game/06_DamageSystem/S_DamageInfo Structure"))
  (returns (WasDamaged :type Boolean)))

(fn `UpdateSpeed`
  (params (NewSpeed :type "Float (double-precision)"))
  (set `FloatingPawnMovement.MaxSpeed` NewSpeed (`self.FloatingPawnMovement`)))

(fn `UserConstructionScript`)