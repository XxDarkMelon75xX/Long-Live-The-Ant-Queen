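; BP_MovingLeaf is a moving leaf platform that travels back and forth between a start and end position from BeginPlay onward.
; Two timelines lerp the Platform component's relative location, one toward EndPos and one back to StartPos.
; Each timeline's Finished event triggers the other, forming an endless ping-pong loop without sweep collision checks.
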(event `self.ReceiveBeginPlay`
  (`self.MovingTO`))

(event `MovingTo`
  (bind (_direction _alpha) (`Timeline|MovingPlatformTo` :!via `PlayFromStart`)
    (:`Update`
      (`SceneComponent.K2_SetRelativeLocation` (`self.Platform`) (`KismetMathLibrary.VLerp` (`self.StartPos`) (`self.EndPos`) _alpha) false false))
    (:`Finished`
      (`self.MovingBack`))))

(event `MovingBack`
  (bind (_direction _alpha) (`Timeline|MovingPlatformBack` :!via `PlayFromStart`)
    (:`Update`
      (`SceneComponent.K2_SetRelativeLocation` (`self.Platform`) (`KismetMathLibrary.VLerp` (`self.EndPos`) (`self.StartPos`) _alpha) false false))
    (:`Finished`
      (`self.MovingTo`))))

(fn `UserConstructionScript`)