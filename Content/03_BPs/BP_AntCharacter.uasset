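; Follower ant character that moves via AI toward the player, taking either an order or one of two follow modes toggled by the player's right click.
; An active order sends it to a reserved location point until recalled; Square mode sends it to its assigned player slot.
; In Free mode, the manager's leader chases the player's follow point while others chase the leader.
; Once the leader arrives, followers stop when enough overlapping neighbours have stopped, spreading the halt through the crowd.
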(event `self.ReceiveBeginPlay`
  (`self.Initialize`)
  (add `/Game/03_BPs/BP_AntPlayer.OnRightClick` (`self.AntPlayer`) (delegate `Handle_RightClick`)))

(event `Handle_RightClick`
  (params (NewParam :type "/Game/03_BPs/Enum_FollowMode Enum" :default "NewEnumerator1"))
  (set `self.FollowMode` NewParam))

(event `self.ReceiveTick`
  (params (DeltaSeconds :type "Float (single-precision)"))
  (if (`self.bHasOrder`)
    (`|AIMoveTo` self (`SceneComponent.K2_GetComponentLocation` (`self.OrderLocationPoint`)) null (`self.OrderAcceptanceRadius`))
    (else
      (switch `/Game/03_BPs/Enum_FollowMode` (`self.FollowMode`)
        (:`NewEnumerator1`
          (if (== (`/Game/03_BPs/BP_AntManager.CurrentLeader` (`self.AntManager`)) self)
            (bind _returnvalue (`self.CheckDistanceToPlayer`))
            (if (not _returnvalue)
              (set `self.bHasReachedDestination` false)
              (`|AIMoveTo` self (`SceneComponent.K2_GetComponentLocation` (`/Game/03_BPs/BP_AntPlayer.FollowPoint` (`self.AntPlayer`))) null (`self.AcceptanceRadius`)
                (:`OnSuccess`
                  (`self.ReachDestination`))))
            (elif (`/Game/03_BPs/BP_AntCharacter.bHasReachedDestination` (`/Game/03_BPs/BP_AntManager.CurrentLeader` (`self.AntManager`)))
              (if (not (`self.bHasReachedDestination`))
                (bind _outactors (`KismetSystemLibrary.SphereOverlapActors` (`self.K2_GetActorLocation`) (`self.DetectionRadius`) (`|MakeArray` "ObjectTypeQuery2" "ObjectTypeQuery3" :!type "EObjectTypeQuery Enum") "BP_AntCharacter_C"))
                (bind _stoppedfollower (`self.CountStoppedFollower` _outactors))
                (if (>= _stoppedfollower (`self.StoppedFollowerNeeded`))
                  (`self.ReachDestination`)))
              (else
                (set `self.bHasReachedDestination` false)
                (`|AIMoveTo` self (0.0 0.0 0.0) (`/Game/03_BPs/BP_AntManager.CurrentLeader` (`self.AntManager`)) (`self.AcceptanceRadiusLeader`)
                  (:`OnSuccess`
                    (`self.ReachDestination`)))))))
        (:`NewEnumerator0`
          (`|AIMoveTo` self (`SceneComponent.K2_GetComponentLocation` (`self.FollowPlayerSquareLocation`)) null (`self.AcceptanceRadius`)))))))

(fn `CheckDistanceToPlayer`
  (returns (ReturnValue :type Boolean))
  (return (<= (`KismetMathLibrary.Vector_Distance` (`SceneComponent.K2_GetComponentLocation` (`/Game/03_BPs/BP_AntPlayer.FollowPoint` (`self.AntPlayer`))) (`self.K2_GetActorLocation`)) (+ (`self.AcceptanceRadius`) 10.0))))

(fn `CountStoppedFollower`
  (params (InputPin :type "Array of Actor Object Reference"))
  (returns (StoppedFollower :type Integer))
  (set `self.StoppedFollowerCount` 0)
  (for _array_element InputPin
    (bind _asbp_ant_character (cast `/Game/03_BPs/BP_AntCharacter` _array_element))
    (if (`/Game/03_BPs/BP_AntCharacter.bHasReachedDestination` _asbp_ant_character)
      (`/Engine/EditorBlueprintResources/StandardMacros.IncrementInt` (`self.StoppedFollowerCount`)
        (:`  `
          (if (>= (`self.StoppedFollowerCount`) (`self.StoppedFollowerNeeded`))
            (break))))))
  (return (`self.StoppedFollowerCount`)))

(fn `Initialize`
  (bind _returnvalue (`GameplayStatics.GetActorOfClass` "/Game/03_BPs/BP_AntManager.BP_AntManager_C"))
  (set `self.AntManager` _returnvalue)
  (bind _returnvalue_2 (`GameplayStatics.GetActorOfClass` "/Game/03_BPs/BP_AntPlayer.BP_AntPlayer_C"))
  (bind _output_get (set `self.AntPlayer` _returnvalue_2))
  (bind _location (`/Game/03_BPs/BP_AntPlayer.GetNewFollowerLocation` _output_get))
  (set `self.FollowPlayerSquareLocation` _location))

(fn `NewFollowOrder`
  (params (Location :type "/Game/03_BPs/Component/BP_FollowerLocationComponent Object Reference"))
  (bind _output_get (set `self.OrderLocationPoint` Location))
  (set `/Game/03_BPs/Component/BP_FollowerLocationComponent.IsOccupied` true _output_get)
  (set `self.bHasOrder` true))

(fn `ReachDestination`
  (set `self.bHasReachedDestination` true)
  (`MovementComponent.StopMovementImmediately` (`self.CharacterMovement`)))

(fn `Recall`
  (bind _orderlocationpoint (`self.OrderLocationPoint`))
  (`/Engine/EditorBlueprintResources/StandardMacros.IsValid` _orderlocationpoint
    (:`Is Valid`
      (set `/Game/03_BPs/Component/BP_FollowerLocationComponent.IsOccupied` false _orderlocationpoint))
    (:`Is Not Valid`
      _))
  (set `self.bHasOrder` false)
  (set `self.OrderLocationPoint` null))

(fn `UserConstructionScript`)