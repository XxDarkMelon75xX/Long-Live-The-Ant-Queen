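; BP_Player is the player pawn, which moves to requested locations via AI and supplies formation slots for followers.
; MoveToLocation sends the pawn to a destination with AIMoveTo.
; GetFollowerLocation returns the first follower location component flagged IsOccupied, otherwise adds one at runtime and increments the count.
; CalculateNewLocation places new slots in a grid relative to FollowPoint, using count, column and row spacing, and player spacing.
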(event `MoveToLocation`
  (params (Location :type "Vector Structure"))
  (`|AIMoveTo` self Location null))

(fn `CalculateNewLocation`
  (returns (Transform :type "Transform Structure"))
  (bind _returnvalue (`SceneComponent.GetRelativeTransform` (`self.FollowPoint`)))
  (return (`KismetMathLibrary.MakeTransform` (`KismetMathLibrary.MakeVector` (- (`self.PlayerSpacing`) (* (- (/ (- (`self.FollowerLocationCount`) (mod (`self.FollowerLocationCount`) (`self.ColumnCount`))) (`self.ColumnCount`)) 1) (`self.RowSpacing`))) (+ (- (.y (.location _returnvalue)) (/ (* (- (`self.ColumnCount`) 1) (`self.ColumnSpacing`)) 2.0)) (* (mod (`self.FollowerLocationCount`) (`self.ColumnCount`)) (`self.ColumnSpacing`))) (.z (.location _returnvalue))) (.rotation _returnvalue) (.scale _returnvalue))))

(fn `GetFollowerLocation`
  (returns (Location :type "/Game/03_BPs/Component/BP_FollowerLocationComponent Object Reference"))
  (for _array_element (`self.K2_GetComponentsByClass` "/Game/03_BPs/Component/BP_FollowerLocationComponent.BP_FollowerLocationComponent_C")
    (if (`/Game/03_BPs/Component/BP_FollowerLocationComponent.IsOccupied` _array_element)
      (return _array_element)))
  (bind _transform (`self.CalculateNewLocation`))
  (bind _returnvalue (`|AddComponentByClass` "/Game/03_BPs/Component/BP_FollowerLocationComponent.BP_FollowerLocationComponent_C" false _transform))
  (`/Engine/EditorBlueprintResources/StandardMacros.IncrementInt` (`self.FollowerLocationCount`)
    (:`  `
      (return _returnvalue))))

(fn `UserConstructionScript`
  (`parent.UserConstructionScript`))