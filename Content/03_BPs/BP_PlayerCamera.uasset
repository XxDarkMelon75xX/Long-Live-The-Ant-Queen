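; Player camera pawn for top-down-style mouse control, which moves and zooms via Enhanced Input and creates the main UI widget.
; Move and zoom feed movement input along the root component's axes.
; The UI's order button toggles OrderMode, which decides whether a left-click cursor trace broadcasts the clicked actor and location or only the location.
; Right-click and the UI recall button are relayed through event dispatchers for other objects to handle.
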(event `self.ReceiveBeginPlay`
  (`self.SetDefaultInput`)
  (bind _returnvalue (`|CreateWidget` "/Game/03_BPs/WBP_UI.WBP_UI_C"))
  (`UserWidget.AddToViewport` _returnvalue 0)
  (add `/Game/03_BPs/WBP_UI.OnOrderButtonClicked` _returnvalue (delegate `OnButtonClicked_Event`))
  (add `/Game/03_BPs/WBP_UI.OnRecallButtonClicked` _returnvalue (delegate `OnRecallClicked_Event`)))

(event `EnhancedInput|/Game/03_BPs/Inputs/IA_Move`
  (params (ActionValue :type "Vector2D Structure") (ElapsedSeconds :type "Float (double-precision)") (TriggeredSeconds :type "Float (double-precision)") (InputAction :type "InputAction Object Reference" :default "/Game/03_BPs/Inputs/IA_Move.IA_Move"))
  (:`Triggered`
    (`self.Move` ActionValue)))

(event `OnRecallClicked_Event`
  (`self.OnRecallClicked`))

(event `OnButtonClicked_Event`
  (set `self.OrderMode` (not (`self.OrderMode`))))

(event `EnhancedInput|/Game/03_BPs/Inputs/IA_Zoom`
  (params (ActionValue :type "Float (double-precision)") (ElapsedSeconds :type "Float (double-precision)") (TriggeredSeconds :type "Float (double-precision)") (InputAction :type "InputAction Object Reference" :default "/Game/03_BPs/Inputs/IA_Zoom.IA_Zoom"))
  (:`Triggered`
    (`self.Zoom` ActionValue)))

(event `EnhancedInput|/Game/03_BPs/Inputs/IA_LeftClick`
  (params (ActionValue :type Boolean) (ElapsedSeconds :type "Float (double-precision)") (TriggeredSeconds :type "Float (double-precision)") (InputAction :type "InputAction Object Reference" :default "/Game/03_BPs/Inputs/IA_LeftClick.IA_LeftClick"))
  (:`Started`
    (`self.LeftClick`)))

(event `EnhancedInput|/Game/03_BPs/Inputs/IA_RightClick`
  (params (ActionValue :type Boolean) (ElapsedSeconds :type "Float (double-precision)") (TriggeredSeconds :type "Float (double-precision)") (InputAction :type "InputAction Object Reference" :default "/Game/03_BPs/Inputs/IA_RightClick.IA_RightClick"))
  (:`Triggered`
    (`self.RightClick`)))

(fn `LeftClick`
  (bind (_bblockinghit _binitialoverlap _time _distance _location _impactpoint _normal _impactnormal _physmat _hitactor) (`GameplayStatics.BreakHitResult` (`PlayerController.GetHitResultUnderCursorByChannel` (`GameplayStatics.GetPlayerController` 0) "TraceTypeQuery1" true)))
  (if (`self.OrderMode`)
    (`self.OnActorClicked` _hitactor _location)
    (else
      (`self.OnLeftClick` (`.Location` (`GameplayStatics.BreakHitResult` (`PlayerController.GetHitResultUnderCursorByChannel` (`GameplayStatics.GetPlayerController` 0) "TraceTypeQuery1" true)))))))

(fn `Move`
  (params (Value :type "Vector2D Structure"))
  (`self.AddMovementInput` (`SceneComponent.GetRightVector` (`self.DefaultSceneRoot`)) Value_X)
  (`self.AddMovementInput` (`SceneComponent.GetForwardVector` (`self.DefaultSceneRoot`)) Value_Y))

(fn `RightClick`
  (`self.OnRightClick`))

(fn `SetDefaultInput`
  (bind _returnvalue (`GameplayStatics.GetPlayerController` 0))
  (bind _returnvalue_2 (pcsubsystem `EnhancedInputLocalPlayerSubsystem` _returnvalue))
  (set `PlayerController.bShowMouseCursor` true _returnvalue)
  (`/Engine/EditorBlueprintResources/StandardMacros.IsValid` _returnvalue_2
    (:`Is Valid`
      (`EnhancedInputSubsystemInterface.AddMappingContext` _returnvalue_2 "/Game/03_BPs/Inputs/IMC_CameraPlayer.IMC_CameraPlayer" 0 (struct)))
    (:`Is Not Valid`
      (`KismetSystemLibrary.PrintString` "Enhanced Input Local Player Subsystem not valid"))))

(fn `UserConstructionScript`)

(fn `Zoom`
  (params (Value :type "Float (double-precision)"))
  (`self.AddMovementInput` (`SceneComponent.GetUpVector` (`self.DefaultSceneRoot`)) (* Value (`self.ZoomFactor`) -1.0)))