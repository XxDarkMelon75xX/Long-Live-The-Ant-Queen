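; A wall actor that ants burn away once enough of them occupy its interact points.
; BeginPlay spawns a row of BP_InteractPoints sized by RequiredAnts, previewed as billboards by the construction script.
; Cursor hover swaps the overlay material, shows the bobbing ant-count widget and notifies BP_RTSPlayerController.
; Reaching the count locks the ants into a fire animation, drives a timeline dissolve material, then frees them and destroys the wall.
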(event `self.ReceiveBeginPlay`
  (bind (_relativelocation_x _relativelocation_y _relativelocation_z) (`KismetMathLibrary.BreakVector` (`SceneComponent.RelativeLocation` (`self.Widget`))))
  (`self.CreateInteractPoints`)
  (`MeshComponent.SetOverlayMaterial` (`self.Cube`) "/Game/_LLTAQ/07_Materials/M_Outline.M_Outline")
  (set `self.BaseZWidget` _relativelocation_z)
  (`self.UpdateAntText`))

(event `self.ReceiveTick`
  (params (DeltaSeconds :type "Float (single-precision)"))
  (`self.MoveWidget` DeltaSeconds))

(event `Burn`
  (`self.ReserveAllAnts`)
  (set `self.HasBurnt` true)
  (`self.EndHover`)
  (`MeshComponent.SetOverlayMaterial` (`self.Cube`) null)
  (`KismetSystemLibrary.Delay` 2.0)
  (bind _returnvalue (`PrimitiveComponent.CreateDynamicMaterialInstance` (`self.Cube`) 0 "/Game/Dissolve/M_Dissolve.M_Dissolve" "None"))
  (bind _output_get (set `self.DissolveMaterial` _returnvalue))
  (`TimelineComponent.SetPlayRate` (`self.Timeline`) (/ 1.0 (`self.TimeToComplete`)))
  (bind (_direction _newtrack_0) (`Timeline|Timeline` :!via `PlayFromStart`)
    (:`Update`
      (`MaterialInstanceDynamic.SetScalarParameterValue` _output_get "Dissolve" _newtrack_0)
      (`PrimitiveComponent.SetCollisionEnabled` (`self.Cube`) "NoCollision"))
    (:`Finished`
      (`self.FreeAllAnts`)
      (`KismetSystemLibrary.DelayUntilNextTick`)
      (`self.K2_DestroyActor`)
      (`GameplayStatics.PlaySound2D` "/Game/08_Audio/SFX/Success.Success" 1.0 1.0 0.0 null null))))

(event `self.Cube.OnBeginCursorOver`
  (params (TouchedComponent :type "PrimitiveComponent Object Reference"))
  (if (not (`self.HasBurnt`))
    (`self.StartHover`)))

(event `self.Cube.OnEndCursorOver`
  (params (TouchedComponent :type "PrimitiveComponent Object Reference"))
  (if (not (`self.HasBurnt`))
    (`self.EndHover`)))

(event `/Game/_LLTAQ/02_Blueprints/BPI_Interaction.AddAnt`
  (`/Engine/EditorBlueprintResources/StandardMacros.IncrementInt` (`self.CurrentAnts`)
    (:`  `
      (`self.UpdateAntText`)
      (`SceneComponent.SetVisibility` (`self.Widget`) true false)
      (`self.CheckBurnable`))))

(event `/Game/_LLTAQ/02_Blueprints/BPI_Interaction.RemoveAnt`
  (`/Engine/EditorBlueprintResources/StandardMacros.DecrementInt` (`self.CurrentAnts`)
    (:`  `
      (`self.UpdateAntText`))))

(fn `CheckBurnable`
  (if (>= (`self.CurrentAnts`) (`self.RequiredAnts`))
    (`self.Burn`)))

(fn `CreateInteractPoints`
  (locals (X :type "Float (double-precision)") (Y :type "Float (double-precision)") (Z :type "Float (double-precision)") (AngleStep :type "Float (double-precision)") (Angle :type "Float (double-precision)") (LineStep :type "Float (double-precision)") (OriginY :type "Float (double-precision)"))
  (if (== (`self.RequiredAnts`) 1)
    (set `local.LineStep` 0.0)
    (set `local.OriginY` 0.0)
    (else
      (set `local.LineStep` (/ (`self.LineLength`) (- (`self.RequiredAnts`) 1)))
      (set `local.OriginY` (/ (`self.LineLength`) 2.0 -1.0))))
  (set `local.X` (`self.DistanceToWall`))
  (set `local.Z` (`self.HeigthOffset`))
  (for _index (range (`self.RequiredAnts`))
    (set `local.Y` (+ (* _index (`local.LineStep`)) (`local.OriginY`)))
    (bind _returnvalue (`|SpawnActorFromClass` "/Game/_LLTAQ/02_Blueprints/BP_InteractPoint.BP_InteractPoint_C" (`SceneComponent.K2_GetComponentToWorld` (`self.HoldPointsRoot`)) "Undefined" "MultiplyWithRoot" null null))
    (`KismetArrayLibrary.Array_Add` (`self.InteractPoints`) _returnvalue)
    (bind _rootcomponent (`Actor.RootComponent` _returnvalue))
    (`SceneComponent.K2_AttachToComponent` _rootcomponent (`self.HoldPointsRoot`) "None" "KeepRelative" "KeepRelative" "KeepRelative" true)
    (`SceneComponent.K2_SetRelativeLocation` _rootcomponent (`KismetMathLibrary.MakeVector` (`local.X`) (`local.Y`) (`local.Z`)) false false)
    (`SceneComponent.K2_SetRelativeRotation` _rootcomponent (struct :`Yaw` 180.0) false false)
    (set `/Game/_LLTAQ/02_Blueprints/BP_InteractPoint.Parent` self _returnvalue)))

(fn `EndHover`
  (set `self.Hovered` false)
  (`MeshComponent.SetOverlayMaterial` (`self.Cube`) "/Game/_LLTAQ/07_Materials/M_Outline.M_Outline")
  (`SceneComponent.SetVisibility` (`self.Widget`) false false)
  (bind _asbp_rtsplayer_controller (cast `/Game/_LLTAQ/02_Blueprints/BP_RTSPlayerController` (`GameplayStatics.GetPlayerController` 0)))
  (`/Game/_LLTAQ/02_Blueprints/BP_RTSPlayerController.SetHoverActor` _asbp_rtsplayer_controller self false))

(fn `FreeAllAnts`
  (for _array_element (`self.InteractPoints`)
    (`/Game/_LLTAQ/02_Blueprints/BP_RTSUnit.DetachFromInteractPoint` (`/Game/_LLTAQ/02_Blueprints/BP_InteractPoint.CurrentUnit` _array_element))))

(fn `GetAntsNeeded`
  (returns (Value :type Integer))
  (return (- (`self.RequiredAnts`) (`self.CurrentAnts`))))

(fn `GetExitPoint`
  (returns (Arrow :type "ArrowComponent Object Reference"))
  (return null))

(fn `GetFreeInteractPoint`
  (returns (Point :type "/Game/_LLTAQ/02_Blueprints/BP_InteractPoint Object Reference"))
  (for _array_element (`self.InteractPoints`)
    (if (not (`/Game/_LLTAQ/02_Blueprints/BP_InteractPoint.bIsOccupied` _array_element))
      (return _array_element)))
  (return null))

(fn `MoveWidget`
  (params (A :type "Float (double-precision)"))
  (set `self.ElapsedTime` (+ A (`self.ElapsedTime`)))
  (`SceneComponent.K2_SetRelativeLocation` (`self.Widget`) (`KismetMathLibrary.MakeVector` 0.0 0.0 (+ (* (`self.FloatAmplitude`) (`KismetMathLibrary.Sin` (* (`self.ElapsedTime`) (`self.FloatSpeed`)))) (`self.BaseZWidget`))) true false))

(fn `ReserveAllAnts`
  (for _array_element (`self.InteractPoints`)
    (bind _currentunit (`/Game/_LLTAQ/02_Blueprints/BP_InteractPoint.CurrentUnit` _array_element))
    (`/Game/_LLTAQ/02_Blueprints/BP_RTSUnit.PlayFireAnimation` _currentunit)
    (`/Game/_LLTAQ/02_Blueprints/BP_RTSUnit.PreventSelection` _currentunit)))

(fn `StartHover`
  (set `self.Hovered` true)
  (`MeshComponent.SetOverlayMaterial` (`self.Cube`) "/Game/_LLTAQ/07_Materials/M_Hover.M_Hover")
  (`SceneComponent.SetVisibility` (`self.Widget`) true false)
  (bind _asbp_rtsplayer_controller (cast `/Game/_LLTAQ/02_Blueprints/BP_RTSPlayerController` (`GameplayStatics.GetPlayerController` 0)))
  (`/Game/_LLTAQ/02_Blueprints/BP_RTSPlayerController.SetHoverActor` _asbp_rtsplayer_controller self true))

(fn `UpdateAntText`
  (bind _aswbp_block_info (cast `/Game/_LLTAQ/06_UI/WBP_BlockInfo` (`WidgetComponent.GetWidget` (`self.Widget`))))
  (`/Game/_LLTAQ/06_UI/WBP_BlockInfo.UpdateText` _aswbp_block_info (`self.CurrentAnts`) (`self.RequiredAnts`)))

(fn `UserConstructionScript`
  (locals (X :type "Float (double-precision)") (Y :type "Float (double-precision)") (Z :type "Float (double-precision)") (LineStep :type "Float (double-precision)") (OriginY :type "Float (double-precision)"))
  (if (== (`self.RequiredAnts`) 1)
    (set `local.LineStep` 0.0)
    (set `local.OriginY` 0.0)
    (else
      (set `local.LineStep` (/ (`self.LineLength`) (- (`self.RequiredAnts`) 1)))
      (set `local.OriginY` (/ (`self.LineLength`) 2.0 -1.0))))
  (set `local.X` (`self.DistanceToWall`))
  (set `local.Z` (`self.HeigthOffset`))
  (for _index (range (`self.RequiredAnts`))
    (set `local.Y` (+ (* _index (`local.LineStep`)) (`local.OriginY`)))
    (bind _returnvalue (`AddComponent|NODE_AddBillboardComponent-0`))
    (`SceneComponent.K2_SetRelativeLocation` _returnvalue (`KismetMathLibrary.MakeVector` (`local.X`) (`local.Y`) (`local.Z`)) false false)))